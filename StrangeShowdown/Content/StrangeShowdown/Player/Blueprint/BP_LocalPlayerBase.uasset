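; Base character for the local player, wiring input, inventory, quick slots, store and stats to the PlayerController's HUD.
; Quick slot 1 arms the gun, which allows toggled aiming via a camera Timeline and movement-rotation swap; other slots use inventory items.
; Firing while aimed directly deducts HP from the player tracked by AttackTraceComp.
; BeginPlay also selects the character mesh and seeds a temporary HealPack store item; debug keys add stamina and gold.
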(event Custom|UpdateInventory
  (bind _playercontroller (Variables|Default|GetPlayerController))
  (bind _player_hud (Variables|/Game/StrangeShowdown/Controller/PC_PlayerController.PC_PlayerController_C|GetPlayer%20HUD _playercontroller))
  (bind _wb_inventorymenu (Variables|/Game/StrangeShowdown/UI/WB_HUD.WB_HUD_C|GetWB_InventoryMenu _player_hud))
  ;[0.15 0.15 0.15 0.5] Inventory
  (Utilities|IsValid _wb_inventorymenu
    (:Is%20Valid
      (Default|UpdateInventory (Variables|/Game/StrangeShowdown/UI/Inventory/WB_InventoryMenu.WB_InventoryMenu_C|GetWB_Inventory _wb_inventorymenu) (Variables|Default|GetInventoryComp)))))

(event Custom|InitializeQuickSlot
  ;[0.15 0.15 0.15 0.5] Inventory
  (Default|InitializeQuickSlot (Variables|/Game/StrangeShowdown/Controller/PC_PlayerController.PC_PlayerController_C|GetPlayer%20HUD (Variables|Default|GetPlayerController)) (Variables|Default|GetQuickSlot%20Comp)))

(event Custom|InitializeStatUI
  (bind _playercontroller (Variables|Default|GetPlayerController))
  (bind _player_hud (Variables|/Game/StrangeShowdown/Controller/PC_PlayerController.PC_PlayerController_C|GetPlayer%20HUD _playercontroller))
  (bind _wb_tabuimenu (Variables|/Game/StrangeShowdown/UI/WB_HUD.WB_HUD_C|GetWB_TabUIMenu _player_hud))
  ;[0.15 0.15 0.15 0.5] Stat UI
  (CallFunction|UpdateAllStat) ; 자신의 UI
  (Utilities|IsValid _wb_tabuimenu
    (:Is%20Valid
      (Default|UpdateTabUI (Variables|/Game/StrangeShowdown/UI/TabUI/WB_TabUIMenu.WB_TabUIMenu_C|GetWB_TabUI _wb_tabuimenu)) ; Tab UI
    )))

(event Custom|UpdateStatUI
  (bind _playercontroller (Variables|Default|GetPlayerController))
  (bind _player_hud (Variables|/Game/StrangeShowdown/Controller/PC_PlayerController.PC_PlayerController_C|GetPlayer%20HUD _playercontroller))
  (bind _wb_tabuimenu (Variables|/Game/StrangeShowdown/UI/WB_HUD.WB_HUD_C|GetWB_TabUIMenu _player_hud))
  ;[0.15 0.15 0.15 0.5] Stat UI
  (CallFunction|UpdateAllStat) ; 자신의 UI
  (Utilities|IsValid _wb_tabuimenu
    (:Is%20Valid
      (Default|UpdateTabUI (Variables|/Game/StrangeShowdown/UI/TabUI/WB_TabUIMenu.WB_TabUIMenu_C|GetWB_TabUI _wb_tabuimenu)) ; Tab UI
    )))

(event Custom|UpdateStore
  (bind _playercontroller (Variables|Default|GetPlayerController))
  (bind _player_hud (Variables|/Game/StrangeShowdown/Controller/PC_PlayerController.PC_PlayerController_C|GetPlayer%20HUD _playercontroller))
  (bind _wb_storemenu (Variables|/Game/StrangeShowdown/UI/WB_HUD.WB_HUD_C|GetWB_StoreMenu _player_hud))
  ;[0.15 0.15 0.15 0.5] Store
  (Utilities|IsValid _wb_storemenu
    (:Is%20Valid
      (Default|UpdateStore (Variables|/Game/StrangeShowdown/UI/Store/WB_StoreMenu.WB_StoreMenu_C|GetWB_Store _wb_storemenu) (Variables|Default|GetStoreComp)))))

(event Custom|ZoomInByAiming
  (bind _charactermovement (Variables|Character|GetCharacterMovement))
  ;[0.15 0.15 0.15 0.5] Zoom Event
  (Variables|Default|SetbIsAiming true)
  (Variables|/Script/Engine.CharacterMovementComponent|SetbUseControllerDesiredRotation _charactermovement true)
  (Variables|/Script/Engine.CharacterMovementComponent|SetbOrientRotationToMovement _charactermovement false)
  (bind (_direction _springarmlength _cameraylocation) (Timeline|Timeline_0 Play)
    (:Update
      (Variables|/Script/Engine.SpringArmComponent|SetTargetArmLength (Variables|Default|GetSpringArmComp) _springarmlength)
      (Transformation|SetRelativeLocation (Variables|Default|GetCameraComp) (Math|Vector|MakeVector 0.0 _cameraylocation 0.0) false false))))

(event Custom|ZoomOutByAiming
  (bind _charactermovement (Variables|Character|GetCharacterMovement))
  ;[0.15 0.15 0.15 0.5] Zoom Event
  (Variables|Default|SetbIsAiming false)
  (Variables|/Script/Engine.CharacterMovementComponent|SetbUseControllerDesiredRotation _charactermovement false)
  (Variables|/Script/Engine.CharacterMovementComponent|SetbOrientRotationToMovement _charactermovement true)
  (bind (_direction _springarmlength _cameraylocation) (Timeline|Timeline_0 Reverse)
    (:Update
      (Variables|/Script/Engine.SpringArmComponent|SetTargetArmLength (Variables|Default|GetSpringArmComp) _springarmlength)
      (Transformation|SetRelativeLocation (Variables|Default|GetCameraComp) (Math|Vector|MakeVector 0.0 _cameraylocation 0.0) false false))))

(event Input|EnhancedActionEvents|EnhancedInputActionIA_LookAround
  (params (ActionValue :type Vector%202D%20Structure) (ElapsedSeconds :type Float%20%28double-precision%29) (TriggeredSeconds :type Float%20%28double-precision%29) (InputAction :type Input%20Action%20Object%20Reference :default "/Game/StrangeShowdown/Input/Actions/IA_LookAround.IA_LookAround"))
  ;[0.15 0.15 0.15 0.5] IA_LookAround
  (Pawn|Input|AddControllerYawInput (.x ActionValue))
  (Pawn|Input|AddControllerPitchInput (* (.y ActionValue) -1.0)))

(event Input|EnhancedActionEvents|EnhancedInputActionIA_Movement
  (params (ActionValue :type Vector%202D%20Structure) (ElapsedSeconds :type Float%20%28double-precision%29) (TriggeredSeconds :type Float%20%28double-precision%29) (InputAction :type Input%20Action%20Object%20Reference :default "/Game/StrangeShowdown/Input/Actions/IA_Movement.IA_Movement"))
  (bind _returnvalue (Pawn|GetControlRotation :!class /Script/Engine.Pawn))
  ;[0.15 0.15 0.15 0.5] IA_Movement
  (Pawn|Input|AddMovementInput (Math|Vector|GetRightVector (Math|Rotator|MakeRotator (.roll _returnvalue) 0.0 (.yaw _returnvalue))) (.x ActionValue) false)
  (Pawn|Input|AddMovementInput (Math|Vector|GetForwardVector (Math|Rotator|MakeRotator 0.0 0.0 (.yaw (Pawn|GetControlRotation :!class /Script/Engine.Pawn)))) (.y ActionValue) false))

(event Input|EnhancedActionEvents|EnhancedInputActionIA_QuickSlot2
  (params (ActionValue :type Boolean) (ElapsedSeconds :type Float%20%28double-precision%29) (TriggeredSeconds :type Float%20%28double-precision%29) (InputAction :type Input%20Action%20Object%20Reference :default "/Game/StrangeShowdown/Input/Actions/IA_QuickSlot2.IA_QuickSlot2"))
  ;[0.15 0.15 0.15 0.5] IA_QuickSlots
  (:Started
    (bind _output_get (Variables|Default|SetCurrentSelectQuickSlotIndex 1))
    (Variables|/Script/StrangeShowdown.STQuickSlotComponent|SetCurrentSelectQuickSlotIndex (Variables|Default|GetQuickSlot%20Comp) _output_get)
    (Variables|Default|SetbIsArmedRifle false)
    (if (Variables|Default|GetbIsAiming)
      (CallFunction|ZoomOutbyAiming))
    (Default|UpdateQuickSlotfromUseItem (Variables|/Game/StrangeShowdown/Controller/PC_PlayerController.PC_PlayerController_C|GetPlayer%20HUD (Variables|Default|GetPlayerController)) (Variables|Default|GetQuickSlot%20Comp))))

(event Input|EnhancedActionEvents|EnhancedInputActionIA_QuickSlot3
  (params (ActionValue :type Boolean) (ElapsedSeconds :type Float%20%28double-precision%29) (TriggeredSeconds :type Float%20%28double-precision%29) (InputAction :type Input%20Action%20Object%20Reference :default "/Game/StrangeShowdown/Input/Actions/IA_QuickSlot3.IA_QuickSlot3"))
  ;[0.15 0.15 0.15 0.5] IA_QuickSlots
  (:Started
    (bind _output_get (Variables|Default|SetCurrentSelectQuickSlotIndex 2))
    (Variables|/Script/StrangeShowdown.STQuickSlotComponent|SetCurrentSelectQuickSlotIndex (Variables|Default|GetQuickSlot%20Comp) _output_get)
    (Variables|Default|SetbIsArmedRifle false)
    (if (Variables|Default|GetbIsAiming)
      (CallFunction|ZoomOutbyAiming))
    (Default|UpdateQuickSlotfromUseItem (Variables|/Game/StrangeShowdown/Controller/PC_PlayerController.PC_PlayerController_C|GetPlayer%20HUD (Variables|Default|GetPlayerController)) (Variables|Default|GetQuickSlot%20Comp))))

(event Input|EnhancedActionEvents|EnhancedInputActionIA_QuickSlot4
  (params (ActionValue :type Boolean) (ElapsedSeconds :type Float%20%28double-precision%29) (TriggeredSeconds :type Float%20%28double-precision%29) (InputAction :type Input%20Action%20Object%20Reference :default "/Game/StrangeShowdown/Input/Actions/IA_QuickSlot4.IA_QuickSlot4"))
  ;[0.15 0.15 0.15 0.5] IA_QuickSlots
  (:Started
    (bind _output_get (Variables|Default|SetCurrentSelectQuickSlotIndex 3))
    (Variables|/Script/StrangeShowdown.STQuickSlotComponent|SetCurrentSelectQuickSlotIndex (Variables|Default|GetQuickSlot%20Comp) _output_get)
    (Variables|Default|SetbIsArmedRifle false)
    (if (Variables|Default|GetbIsAiming)
      (CallFunction|ZoomOutbyAiming))
    (Default|UpdateQuickSlotfromUseItem (Variables|/Game/StrangeShowdown/Controller/PC_PlayerController.PC_PlayerController_C|GetPlayer%20HUD (Variables|Default|GetPlayerController)) (Variables|Default|GetQuickSlot%20Comp))))

(event Input|EnhancedActionEvents|EnhancedInputActionIA_QuickSlot5
  (params (ActionValue :type Boolean) (ElapsedSeconds :type Float%20%28double-precision%29) (TriggeredSeconds :type Float%20%28double-precision%29) (InputAction :type Input%20Action%20Object%20Reference :default "/Game/StrangeShowdown/Input/Actions/IA_QuickSlot5.IA_QuickSlot5"))
  ;[0.15 0.15 0.15 0.5] IA_QuickSlots
  (:Started
    (bind _output_get (Variables|Default|SetCurrentSelectQuickSlotIndex 4))
    (Variables|/Script/StrangeShowdown.STQuickSlotComponent|SetCurrentSelectQuickSlotIndex (Variables|Default|GetQuickSlot%20Comp) _output_get)
    (Variables|Default|SetbIsArmedRifle false)
    (if (Variables|Default|GetbIsAiming)
      (CallFunction|ZoomOutbyAiming))
    (Default|UpdateQuickSlotfromUseItem (Variables|/Game/StrangeShowdown/Controller/PC_PlayerController.PC_PlayerController_C|GetPlayer%20HUD (Variables|Default|GetPlayerController)) (Variables|Default|GetQuickSlot%20Comp))))

(event Input|EnhancedActionEvents|EnhancedInputActionIA_Pickup
  (params (ActionValue :type Boolean) (ElapsedSeconds :type Float%20%28double-precision%29) (TriggeredSeconds :type Float%20%28double-precision%29) (InputAction :type Input%20Action%20Object%20Reference :default "/Game/StrangeShowdown/Input/Actions/IA_Pickup.IA_Pickup"))
  ;[0.15 0.15 0.15 0.5] IA_Pickup
  (:Started
    (bind _outaddedinventoryindex (Class|STLocalPlayer|Interact))
    (CallFunction|UpdateInventory)
    (Class|STQuickSlotComponent|AddtoQuickSlot (Variables|Default|GetQuickSlot%20Comp) (Variables|Default|GetInventoryComp) _outaddedinventoryindex -2) ; -2면 즉시 추가
    (Default|UpdateQuickSlot (Variables|/Game/StrangeShowdown/Controller/PC_PlayerController.PC_PlayerController_C|GetPlayer%20HUD (Variables|Default|GetPlayerController)))))

(event Input|EnhancedActionEvents|EnhancedInputActionIA_GunAiming
  (params (ActionValue :type Boolean) (ElapsedSeconds :type Float%20%28double-precision%29) (TriggeredSeconds :type Float%20%28double-precision%29) (InputAction :type Input%20Action%20Object%20Reference :default "/Game/StrangeShowdown/Input/Actions/IA_GunAiming.IA_GunAiming"))
  ;[0.15 0.15 0.15 0.5] IA_Aiming
  (if (Variables|Default|GetbIsArmedRifle)
    (if (Variables|Default|GetbIsAiming)
      (CallFunction|ZoomOutbyAiming)
      (else
        (CallFunction|ZoominbyAiming)))))

(event Input|EnhancedActionEvents|EnhancedInputActionIA_QuickSlot1
  (params (ActionValue :type Boolean) (ElapsedSeconds :type Float%20%28double-precision%29) (TriggeredSeconds :type Float%20%28double-precision%29) (InputAction :type Input%20Action%20Object%20Reference :default "/Game/StrangeShowdown/Input/Actions/IA_QuickSlot1.IA_QuickSlot1"))
  ;[0.15 0.15 0.15 0.5] IA_QuickSlots
  (:Started
    (bind _output_get (Variables|Default|SetCurrentSelectQuickSlotIndex 0))
    (Variables|/Script/StrangeShowdown.STQuickSlotComponent|SetCurrentSelectQuickSlotIndex (Variables|Default|GetQuickSlot%20Comp) _output_get)
    (Variables|Default|SetbIsArmedRifle true)
    (Default|UpdateQuickSlotfromUseItem (Variables|/Game/StrangeShowdown/Controller/PC_PlayerController.PC_PlayerController_C|GetPlayer%20HUD (Variables|Default|GetPlayerController)) (Variables|Default|GetQuickSlot%20Comp))))

(event Input|EnhancedActionEvents|EnhancedInputActionIA_GunFire
  (params (ActionValue :type Boolean) (ElapsedSeconds :type Float%20%28double-precision%29) (TriggeredSeconds :type Float%20%28double-precision%29) (InputAction :type Input%20Action%20Object%20Reference :default "/Game/StrangeShowdown/Input/Actions/IA_GunFire.IA_GunFire"))
  ;[0.15 0.15 0.15 0.5] IA_GunFire
  (if (Variables|Default|GetbIsArmedRifle) ; 0번(퀵슬롯 1번)이면 공격, 아니면 아이템 사용
    (if (Variables|Default|GetbIsAiming)
      (Utilities|IsValid (Variables|/Script/StrangeShowdown.STAttackTraceComponent|GetTracingFieldPlayer (Variables|Default|GetAttackTraceComp))
        (:Is%20Valid
          (CallFunction|PlayMuzzleFlash)
          (Class|STStatComponent|AddHp (Variables|/Script/StrangeShowdown.STPlayerBase|GetStatComp (Variables|/Script/StrangeShowdown.STAttackTraceComponent|GetTracingFieldPlayer (Variables|Default|GetAttackTraceComp))) -1)
          (bind _asbp_field_player (Utilities|Casting|CastToBP_FieldPlayer (Variables|/Script/StrangeShowdown.STAttackTraceComponent|GetTracingFieldPlayer (Variables|Default|GetAttackTraceComp))))
          (Default|UpdateAllStat _asbp_field_player)
          (Animation|PlayAnimMontage "/Game/PolygonWestern/EpicContent/Mannequin/RetargetAnimations/Pistol/MM_Pistol_Fire_Montage.MM_Pistol_Fire_Montage" 1.0 "None"))))
    (else
      (bind (_outslot _returnvalue) (Class|STInventoryComponent|UseItem (Variables|Default|GetInventoryComp) (Utilities|Array|Get(acopy) (Variables|/Script/StrangeShowdown.STQuickSlotComponent|GetInventorySlotIndex (Variables|Default|GetQuickSlot%20Comp)) (Variables|Default|GetCurrentSelectQuickSlotIndex)) self))
      (if _returnvalue
        (bind _returnvalue_2 (UserInterface|CreateWidget "/Game/StrangeShowdown/Item/Blueprint/WB_UseEffectFloatingMessage.WB_UseEffectFloatingMessage_C"))
        (UserInterface|Viewport|AddtoViewport _returnvalue_2 100)
        (Class|UserWidget|SetPositioninViewport _returnvalue_2 "(X=500.000000,Y=200.000000)" true)
        (Rendering|Components|TextRender|SetText (Variables|/Game/StrangeShowdown/Item/Blueprint/WB_UseEffectFloatingMessage.WB_UseEffectFloatingMessage_C|GetMessage _returnvalue_2) (Variables|/Script/StrangeShowdown.STItemDataAssetBase|GetItemName (.ItemData (Utilities|Struct|BreakInventorySlot _outslot))))
        (Default|UpdateQuickSlotfromUseItem (Variables|/Game/StrangeShowdown/Controller/PC_PlayerController.PC_PlayerController_C|GetPlayer%20HUD (Variables|Default|GetPlayerController)) (Variables|Default|GetQuickSlot%20Comp))))))

(event EventBeginPlay
  (bind _storecomp (Variables|Default|GetStoreComp))
  ;[0.15 0.15 0.15 0.5] BeginPlay
  (bind _aspc_player_controller (Utilities|Casting|CastToPC_PlayerController (Pawn|GetController)))
  (bind _output_get (Variables|Default|SetPlayerController _aspc_player_controller))
  (Input|AddMappingContext (PlayerController|LocalPlayerSubsystems|GetEnhancedInputLocalPlayerSubsystem _output_get) "/Game/StrangeShowdown/Input/IMC_PlayerBaseInput.IMC_PlayerBaseInput" 0 "(bIgnoreAllPressedKeysUntilRelease=True,bForceImmediately=False,bNotifyUserSettings=False)")
  (CallFunction|InitializeQuickSlot)
  (CallFunction|InitializeStatUI)
  (CallFunction|PlayerMeshSelect)
  (Utilities|Array|SetArrayElem (Variables|/Script/StrangeShowdown.STStoreComponent|GetStoreItemPool _storecomp) 0 "/Game/StrangeShowdown/Item/DataAsset/DA_HealPack.DA_HealPack") ; 임시용 0번 아이템: HealPack
  (Class|STStoreComponent|InitStore _storecomp)
  (Variables|/Script/StrangeShowdown.STAttackTraceComponent|SetAttackTraceWidgetClass (Variables|Default|GetAttackTraceComp) "/Game/StrangeShowdown/UI/AttackTrace/WB_AttackTrace.WB_AttackTrace_C"))

(event Input|KeyboardEvents|DebugKey9
  (params (Key :type Key%20Structure :default "None") (ActionValue :type Input%20Action%20Value%20Structure))
  (bind _statcomp (Variables|Default|GetStatComp))
  ;[0.15 0.15 0.15 0.5] Debug Key
  (:Pressed
    (Class|STStatComponent|AddGold _statcomp 1)
    (Development|PrintString (Utilities|String|Append "Gold: " (Utilities|String|ToString(Integer) (Variables|/Script/StrangeShowdown.STStatComponent|GetGold _statcomp))))
    (CallFunction|UpdateStatUI)))

(event Input|KeyboardEvents|DebugKey0
  (params (Key :type Key%20Structure :default "None") (ActionValue :type Input%20Action%20Value%20Structure))
  (bind _statcomp (Variables|Default|GetStatComp))
  ;[0.15 0.15 0.15 0.5] Debug Key
  (:Pressed
    (Class|STStatComponent|AddStamina _statcomp 1)
    (Development|PrintString (Utilities|String|Append "Stamina: " (Utilities|String|ToString(Float) (Variables|/Script/StrangeShowdown.STStatComponent|GetStamina _statcomp))))
    (CallFunction|UpdateStatUI)))

(fn ConstructionScript)

(fn UpdateAllStat
  (bind _playercontroller (Variables|Default|GetPlayerController))
  (bind _statcomp (Variables|Default|GetStatComp))
  (bind _player_hud (Variables|/Game/StrangeShowdown/Controller/PC_PlayerController.PC_PlayerController_C|GetPlayer%20HUD _playercontroller))
  (bind _wb_stat (Variables|/Game/StrangeShowdown/UI/WB_HUD.WB_HUD_C|GetWB_Stat _player_hud))
  (Default|UpdateActionUI _wb_stat _statcomp)
  (Default|UpdateGoldUI _wb_stat _statcomp)
  (Default|UpdateStaminaUI _wb_stat _statcomp)
  (Default|UpdateStatUI _wb_stat _statcomp)
  (Default|UpdateArmorUI _wb_stat _statcomp))

(fn PlayerMeshSelect
  (switch Utilities|FlowControl|Switch|SwitchonEPlayerMeshType (Variables|Default|GetPlayerMeshType)
    (:Badguy
      (Components|SkeletalMesh|SetSkeletalMeshAsset (Variables|Character|GetMesh) "/Game/PolygonWestern/Meshes/CharactersUE4Mannequin/SK_Chr_Badguy_01.SK_Chr_Badguy_01"))
    (:Cowboy
      (Components|SkeletalMesh|SetSkeletalMeshAsset (Variables|Character|GetMesh) "/Game/PolygonWestern/Meshes/CharactersUE4Mannequin/SK_Chr_Cowboy_01.SK_Chr_Cowboy_01"))
    (:Cowgirl
      (Components|SkeletalMesh|SetSkeletalMeshAsset (Variables|Character|GetMesh) "/Game/PolygonWestern/Meshes/CharactersUE4Mannequin/SK_Chr_Cowgirl_01.SK_Chr_Cowgirl_01"))
    (:Gunman
      (Components|SkeletalMesh|SetSkeletalMeshAsset (Variables|Character|GetMesh) "/Game/PolygonWestern/Meshes/CharactersUE4Mannequin/SK_Chr_Gunman_01.SK_Chr_Gunman_01"))))

(fn PlayMuzzleFlash
  (bind _rightweapon (Variables|Default|GetRightWeapon))
  (Niagara|SpawnSystematLocation "/Game/StrangeShowdown/Item/FX/NS_PistolMuzzleFlash.NS_PistolMuzzleFlash" (Transformation|GetSocketLocation _rightweapon "Muzzle") (Transformation|GetSocketRotation _rightweapon "Muzzle")))