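; BP_FieldPlayer is the field player character Blueprint, handling character mesh selection and a stat widget.
; On BeginPlay it caches the widget component's WB_FieldPlayerStatUI and sets one of four western-themed skeletal meshes from PlayerMeshType.
; It defers the first stat refresh until the widget fires its UI-ready event.
; Initial and later refreshes share UpdateAllStat, which passes StatComp to the action, stat, stamina and prize UI updates.
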(event `self.ReceiveBeginPlay`
  (bind _aswb_field_player_stat_ui (cast `/Game/StrangeShowdown/UI/Interfaces/WB_FieldPlayerStatUI` (`WidgetComponent.GetUserWidgetObject` (`self.StatWidgetComponent`))))
  (set `self.StatUI` _aswb_field_player_stat_ui)
  (`self.PlayerMeshSelect`)
  (add `/Game/StrangeShowdown/UI/Interfaces/WB_FieldPlayerStatUI.OnUIReady` (`self.StatUI`) (delegate `UIReady`)))

(event `UIReady`
  (`self.InitializeStatUI`) ; UI 생성이 완료된 후 호출해야 할 필요가 있음
)

(event `InitializeStatUI`
  ; Stat UI
  (`self.UpdateAllStat` :!label _label))

(event `UpdateStatUI`
  ; Stat UI
  (goto _label))

(fn `PlayerMeshSelect`
  (switch `EPlayerMeshType` (`self.PlayerMeshType`)
    (:`Badguy`
      (`SkeletalMeshComponent.SetSkeletalMeshAsset` (`self.Mesh`) "/Game/PolygonWestern/Meshes/CharactersUE4Mannequin/SK_Chr_Badguy_01.SK_Chr_Badguy_01"))
    (:`Cowboy`
      (`SkeletalMeshComponent.SetSkeletalMeshAsset` (`self.Mesh`) "/Game/PolygonWestern/Meshes/CharactersUE4Mannequin/SK_Chr_Cowboy_01.SK_Chr_Cowboy_01"))
    (:`Cowgirl`
      (`SkeletalMeshComponent.SetSkeletalMeshAsset` (`self.Mesh`) "/Game/PolygonWestern/Meshes/CharactersUE4Mannequin/SK_Chr_Cowgirl_01.SK_Chr_Cowgirl_01"))
    (:`Gunman`
      (`SkeletalMeshComponent.SetSkeletalMeshAsset` (`self.Mesh`) "/Game/PolygonWestern/Meshes/CharactersUE4Mannequin/SK_Chr_Gunman_01.SK_Chr_Gunman_01"))))

(fn `UpdateAllStat`
  (bind _statui (`self.StatUI`))
  (bind _statcomp (`self.StatComp`))
  (`/Game/StrangeShowdown/UI/Interfaces/WB_FieldPlayerStatUI.UpdateActionUI` _statui _statcomp)
  (`/Game/StrangeShowdown/UI/Interfaces/WB_FieldPlayerStatUI.UpdateStatUI` _statui _statcomp)
  (`/Game/StrangeShowdown/UI/Interfaces/WB_FieldPlayerStatUI.UpdateStaminaUI` _statui _statcomp)
  (`/Game/StrangeShowdown/UI/Interfaces/WB_FieldPlayerStatUI.UpdatePrizeUI` _statui _statcomp))

(fn `UserConstructionScript`)