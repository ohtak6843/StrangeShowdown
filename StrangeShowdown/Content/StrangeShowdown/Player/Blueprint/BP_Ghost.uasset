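; BP_Ghost is a player ghost Blueprint that shows a nickname and stats through a field stat widget component.
; It waits for the widget's ready event, then fills it from StatComp and binds to the player controller's Shift-hold events.
; Holding Shift shows stamina, prize, gold and action elements, and releasing hides them.
; EndPlay unbinds those controller events, and UpdateStatUI reruns the full stat refresh.
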(event `self.ReceiveEndPlay`
  (params (EndPlayReason :type "EEndPlayReason Enum" :default "Destroyed"))
  ; EndPlay
  (bind _aspc_player_controller (cast `/Game/StrangeShowdown/Controller/PC_PlayerController` (`GameplayStatics.GetPlayerController` 0)))
  (remove `/Game/StrangeShowdown/Controller/PC_PlayerController.OnShiftHoldStart` _aspc_player_controller (delegate `OnShiftHoldStart`)) ; 객체가 소멸할 때 반드시 바인드 한 이벤트를 언바인드
  (remove `/Game/StrangeShowdown/Controller/PC_PlayerController.OnShiftHoldEnd` _aspc_player_controller (delegate `OnShiftHoldEnd`)))

(event `self.ReceiveBeginPlay`
  ; BeginPlay
  (bind _aswb_field_player_stat_ui (cast `/Game/StrangeShowdown/UI/Interfaces/WB_FieldPlayerStatUI` (`WidgetComponent.GetUserWidgetObject` (`self.StatWidgetComponent`))))
  (set `self.StatUI` _aswb_field_player_stat_ui)
  (`TextBlock.SetText` (`/Game/StrangeShowdown/UI/Interfaces/WB_FieldPlayerStatUI.Nickname` (`self.StatUI`)) (`KismetTextLibrary.Conv_StringToText` (`self.PlayerNickName`)))
  (add `/Game/StrangeShowdown/UI/Interfaces/WB_FieldPlayerStatUI.OnUIReady` (`self.StatUI`) (delegate `UIReady`)))

(event `UIReady`
  ; BeginPlay
  (`self.InitializeStatUI`) ; UI 생성이 완료된 후 호출해야 할 필요가 있음
  (bind _aspc_player_controller (cast `/Game/StrangeShowdown/Controller/PC_PlayerController` (`GameplayStatics.GetPlayerController` 0)))
  (add `/Game/StrangeShowdown/Controller/PC_PlayerController.OnShiftHoldStart` _aspc_player_controller (delegate `OnShiftHoldStart`))
  (add `/Game/StrangeShowdown/Controller/PC_PlayerController.OnShiftHoldEnd` _aspc_player_controller (delegate `OnShiftHoldEnd`)))

(event `OnShiftHoldStart`
  ; BeginPlay
  (set `self.bOnShiftPressed` true)
  (`self.ShowShiftUI`))

(event `OnShiftHoldEnd`
  ; BeginPlay
  (set `self.bOnShiftPressed` false)
  (`self.HiddenShiftUI`))

(event `InitializeStatUI`
  ; Stat UI
  (`self.UpdateAllStat` :!label _label))

(event `UpdateStatUI`
  ; Stat UI
  (goto _label))

(fn `HiddenShiftUI`
  (`Widget.SetVisibility` (`/Game/StrangeShowdown/UI/Interfaces/WB_FieldPlayerStatUI.Stamina` (`self.StatUI`)) "Hidden")
  (`Widget.SetVisibility` (`/Game/StrangeShowdown/UI/Interfaces/WB_FieldPlayerStatUI.Prize` (`self.StatUI`)) "Hidden")
  (`Widget.SetVisibility` (`/Game/StrangeShowdown/UI/Interfaces/WB_FieldPlayerStatUI.GoldImage` (`self.StatUI`)) "Hidden")
  (`Widget.SetVisibility` (`/Game/StrangeShowdown/UI/Interfaces/WB_FieldPlayerStatUI.ActionNum` (`self.StatUI`)) "Hidden")
  (`Widget.SetVisibility` (`/Game/StrangeShowdown/UI/Interfaces/WB_FieldPlayerStatUI.ActionImage` (`self.StatUI`)) "Hidden"))

(fn `ShowShiftUI`
  (`Widget.SetVisibility` (`/Game/StrangeShowdown/UI/Interfaces/WB_FieldPlayerStatUI.Stamina` (`self.StatUI`)) "Visible")
  (`Widget.SetVisibility` (`/Game/StrangeShowdown/UI/Interfaces/WB_FieldPlayerStatUI.Prize` (`self.StatUI`)) "Visible")
  (`Widget.SetVisibility` (`/Game/StrangeShowdown/UI/Interfaces/WB_FieldPlayerStatUI.GoldImage` (`self.StatUI`)) "Visible")
  (`Widget.SetVisibility` (`/Game/StrangeShowdown/UI/Interfaces/WB_FieldPlayerStatUI.ActionNum` (`self.StatUI`)) "Visible")
  (`Widget.SetVisibility` (`/Game/StrangeShowdown/UI/Interfaces/WB_FieldPlayerStatUI.ActionImage` (`self.StatUI`)) "Visible"))

(fn `UpdateAllStat`
  (bind _statui (`self.StatUI`))
  (bind _statcomp (`self.StatComp`))
  (`/Game/StrangeShowdown/UI/Interfaces/WB_FieldPlayerStatUI.UpdateStatUI` _statui _statcomp)
  (`/Game/StrangeShowdown/UI/Interfaces/WB_FieldPlayerStatUI.UpdatePrizeUI` _statui _statcomp)
  (`/Game/StrangeShowdown/UI/Interfaces/WB_FieldPlayerStatUI.UpdateActionUI` _statui _statcomp)
  (`/Game/StrangeShowdown/UI/Interfaces/WB_FieldPlayerStatUI.UpdateStaminaUI` _statui _statcomp))

(fn `UserConstructionScript`)