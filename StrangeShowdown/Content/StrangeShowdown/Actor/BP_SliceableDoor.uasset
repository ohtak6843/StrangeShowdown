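; BP_SliceableDoor is a door actor that breaks apart when sliced.
; On the OnSliced event it hides the intact mesh, plays a wood-break sound and reveals the GCSliceableDoor component with physics and collision damage enabled, apparently a Geometry Collection fracture.
; After a short delay it hides the debris and disables collision on both components, leaving the doorway clear.
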(event `self.OnSliced`
  (bind _gc_sliceabledoor (`self.GC_SliceableDoor`))
  (bind _gc_sliceabledoor_2 (`self.GC_SliceableDoor`))
  (`SceneComponent.SetVisibility` (`self.MeshComponent`) false false)
  (`GameplayStatics.SpawnSound2D` "/Game/StrangeShowdown/Sound/Effect/SW_WoodBreak.SW_WoodBreak" 1.0 1.0 0.1 null)
  (`SceneComponent.SetHiddenInGame` _gc_sliceabledoor_2 false false)
  (`GeometryCollectionComponent.SetEnableDamageFromCollision` _gc_sliceabledoor_2 true)
  (`PrimitiveComponent.SetSimulatePhysics` _gc_sliceabledoor_2 true)
  (`KismetSystemLibrary.Delay` 2.0)
  (`SceneComponent.SetHiddenInGame` _gc_sliceabledoor true false)
  (`PrimitiveComponent.SetCollisionEnabled` _gc_sliceabledoor "NoCollision")
  (`PrimitiveComponent.SetCollisionEnabled` (`self.MeshComponent`) "NoCollision"))

(fn `UserConstructionScript`)