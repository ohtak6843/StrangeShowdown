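; BP_GhostController is a player controller that owns the player HUD and handles its UI input.
; On BeginPlay it creates WB_HUD, adds it to the viewport and caches the BP_LocalPlayer pawn.
; Enhanced Input actions toggle the tab menu and big map, with RemoveAllUI closing any open panel before another opens.
; A chat action switches to Game and UI input mode and focuses the chat input box.
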(event `self.ReceiveBeginPlay`
  ; BeginPlay
  (bind _returnvalue (`|CreateWidget` "/Game/StrangeShowdown/UI/WB_HUD.WB_HUD_C" null null))
  (bind _output_get (set `self.HUDWidget` _returnvalue))
  (bind _aswb_hud (cast `/Game/StrangeShowdown/UI/WB_HUD` _output_get))
  (bind _output_get_2 (set `self.Player HUD` _aswb_hud))
  (`UserWidget.AddToViewport` _output_get_2 0)
  (bind _asbp_local_player (cast `/Game/StrangeShowdown/Character/Player/BP_LocalPlayer` (`GameplayStatics.GetPlayerPawn` 0)))
  (set `self.LocalPlayer` _asbp_local_player))

(event `EnhancedInput|/Game/StrangeShowdown/Input/Actions/IA_TabUI`
  (params (ActionValue :type Boolean) (ElapsedSeconds :type "Float (double-precision)") (TriggeredSeconds :type "Float (double-precision)") (InputAction :type "InputAction Object Reference" :default "/Game/StrangeShowdown/Input/Actions/IA_TabUI.IA_TabUI"))
  ; IA_TabUI
  (:`Started`
    (if (not (`self.IsTabUIOpen`))
      (`self.RemoveAllUI`)
      (`/Game/StrangeShowdown/UI/WB_HUD.ShowTabUIMenu` (`self.Player HUD`))
      (set `self.IsTabUIOpen` true)
      (else
        (`/Game/StrangeShowdown/UI/WB_HUD.RemoveTabUIMenu` (`self.Player HUD`))
        (set `self.IsTabUIOpen` false)))))

(event `EnhancedInput|/Game/StrangeShowdown/Input/Actions/IA_FocusChatManager`
  (params (ActionValue :type Boolean) (ElapsedSeconds :type "Float (double-precision)") (TriggeredSeconds :type "Float (double-precision)") (InputAction :type "InputAction Object Reference" :default "/Game/StrangeShowdown/Input/Actions/IA_FocusChatManager.IA_FocusChatManager"))
  ; IA_FocusChatManager
  (:`Started`
    (`WidgetBlueprintLibrary.SetInputMode_GameAndUIEx` self null)
    (`Widget.SetKeyboardFocus` (`STChatManagerWidget.ChatInputTextBox` (`STHUD.ChatManagerWidget` (`self.Player HUD`))))))

(event `EnhancedInput|/Game/StrangeShowdown/Input/Actions/IA_BigMap`
  (params (ActionValue :type Boolean) (ElapsedSeconds :type "Float (double-precision)") (TriggeredSeconds :type "Float (double-precision)") (InputAction :type "InputAction Object Reference" :default "/Game/StrangeShowdown/Input/Actions/IA_BigMap.IA_BigMap"))
  ; IA_BigMap
  (:`Started`
    (if (not (`self.IsBigMapOpen`))
      (`self.RemoveAllUI`)
      (`/Game/StrangeShowdown/UI/WB_HUD.ShowBigMap` (`self.Player HUD`))
      (set `self.IsBigMapOpen` true)
      (else
        (`/Game/StrangeShowdown/UI/WB_HUD.RemoveBigMap` (`self.Player HUD`))
        (set `self.IsBigMapOpen` false)))))

(fn `RemoveAllUI`
  (if (`self.IsTabUIOpen`)
    (`/Game/StrangeShowdown/UI/WB_HUD.RemoveTabUIMenu` (`self.Player HUD`))
    (set `self.IsTabUIOpen` false))
  (if (`self.IsBigMapOpen`)
    (`/Game/StrangeShowdown/UI/WB_HUD.RemoveBigMap` (`self.Player HUD`))
    (set `self.IsBigMapOpen` false)))

(fn `UserConstructionScript`)