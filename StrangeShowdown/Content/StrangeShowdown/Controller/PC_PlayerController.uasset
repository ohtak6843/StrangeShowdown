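; Player controller for Strange Showdown that creates the HUD on BeginPlay and handles UI input.
; Inventory, Store and Tab inputs toggle their HUD menus, with open flags and RemoveAllUI keeping only one open at a time.
; Holding the ShiftUI input broadcasts start and end dispatchers and calls the cached local player's look-up zoom in and out.
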(event `self.ReceiveBeginPlay`
  ; BeginPlay
  (bind _returnvalue (`|CreateWidget` "/Game/StrangeShowdown/UI/WB_HUD.WB_HUD_C" null null))
  (bind _output_get (set `self.Player HUD` _returnvalue))
  (`UserWidget.AddToViewport` _output_get 0)
  (bind _asbp_local_player_base (cast `/Game/StrangeShowdown/Player/Blueprint/BP_LocalPlayerBase` (`GameplayStatics.GetPlayerPawn` 0)))
  (set `self.LocalPlayer` _asbp_local_player_base))

(event `EnhancedInput|/Game/StrangeShowdown/Input/Actions/IA_Inventory`
  (params (ActionValue :type Boolean) (ElapsedSeconds :type "Float (double-precision)") (TriggeredSeconds :type "Float (double-precision)") (InputAction :type "InputAction Object Reference" :default "/Game/StrangeShowdown/Input/Actions/IA_Inventory.IA_Inventory"))
  ; IA_Inventory
  (:`Started`
    (if (not (`self.IsInventoryOpen`))
      (`self.RemoveAllUI`)
      (`/Game/StrangeShowdown/UI/WB_HUD.ShowInventoryMenu` (`self.Player HUD`))
      (set `self.IsInventoryOpen` true)
      (else
        (`/Game/StrangeShowdown/UI/WB_HUD.RemoveInventoryMenu` (`self.Player HUD`))
        (set `self.IsInventoryOpen` false)))))

(event `EnhancedInput|/Game/StrangeShowdown/Input/Actions/IA_Store`
  (params (ActionValue :type Boolean) (ElapsedSeconds :type "Float (double-precision)") (TriggeredSeconds :type "Float (double-precision)") (InputAction :type "InputAction Object Reference" :default "/Game/StrangeShowdown/Input/Actions/IA_Store.IA_Store"))
  ; IA_Store
  (:`Started`
    (if (not (`self.IsStoreOpen`))
      (`self.RemoveAllUI`)
      (`/Game/StrangeShowdown/UI/WB_HUD.ShowStoreMenu` (`self.Player HUD`) (`self.LocalPlayer`))
      (set `self.IsStoreOpen` true)
      (else
        (`/Game/StrangeShowdown/UI/WB_HUD.RemoveStoreMenu` (`self.Player HUD`))
        (set `self.IsStoreOpen` false)))))

(event `EnhancedInput|/Game/StrangeShowdown/Input/Actions/IA_TabUI`
  (params (ActionValue :type Boolean) (ElapsedSeconds :type "Float (double-precision)") (TriggeredSeconds :type "Float (double-precision)") (InputAction :type "InputAction Object Reference" :default "/Game/StrangeShowdown/Input/Actions/IA_TabUI.IA_TabUI"))
  ; IA_TabUI
  (:`Started`
    (if (not (`self.IsTabUIOpen`))
      (`self.RemoveAllUI`)
      (`/Game/StrangeShowdown/UI/WB_HUD.ShowTabUIMenu` (`self.Player HUD`))
      (set `self.IsTabUIOpen` true)
      (else
        (`/Game/StrangeShowdown/UI/WB_HUD.RemoveTabUIMenu` (`self.Player HUD`))
        (set `self.IsTabUIOpen` false)))))

(event `EnhancedInput|/Game/StrangeShowdown/Input/Actions/IA_ShiftUI`
  (params (ActionValue :type Boolean) (ElapsedSeconds :type "Float (double-precision)") (TriggeredSeconds :type "Float (double-precision)") (InputAction :type "InputAction Object Reference" :default "/Game/StrangeShowdown/Input/Actions/IA_ShiftUI.IA_ShiftUI"))
  ; IA_ShiftUI
  (:`Started`
    (`self.OnShiftHoldStart`) ; Shift Pressed에 연결된 모든 이벤트 실행(브로드캐스트)
    (`/Game/StrangeShowdown/Player/Blueprint/BP_LocalPlayerBase.ZoomInByLookingUp` (`self.LocalPlayer`)))
  (:`Completed`
    (`self.OnShiftHoldEnd`)
    (`/Game/StrangeShowdown/Player/Blueprint/BP_LocalPlayerBase.ZoomOutByLookingUp` (`self.LocalPlayer`))))

(fn `RemoveAllUI`
  (if (`self.IsInventoryOpen`)
    (`/Game/StrangeShowdown/UI/WB_HUD.RemoveInventoryMenu` (`self.Player HUD`))
    (set `self.IsInventoryOpen` false))
  (if (`self.IsStoreOpen`)
    (`/Game/StrangeShowdown/UI/WB_HUD.RemoveStoreMenu` (`self.Player HUD`))
    (set `self.IsStoreOpen` false))
  (if (`self.IsTabUIOpen`)
    (`/Game/StrangeShowdown/UI/WB_HUD.RemoveTabUIMenu` (`self.Player HUD`))
    (set `self.IsTabUIOpen` false)))

(fn `UserConstructionScript`)