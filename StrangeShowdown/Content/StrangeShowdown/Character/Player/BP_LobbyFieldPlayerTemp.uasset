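; Temporary lobby field player that shows a selected character mesh with a nickname widget in Strange Showdown.
; PlayerMeshSelect maps PlayerMeshType to one of the western-themed skeletal meshes, such as cowboy, gunman or businessman.
; BeginPlay applies the mesh, caches the stat UI from StatWidgetComponent and writes PlayerNickName into it.
; The mesh selection runs again after the widget cast succeeds.
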(event `self.ReceiveBeginPlay`
  ; BeginPlay
  (`self.PlayerMeshSelect`)
  (bind _aswb_lobby_field_player_stat_ui (cast `/Game/StrangeShowdown/UI/Interfaces/WB_LobbyFieldPlayerStatUI` (`WidgetComponent.GetUserWidgetObject` (`self.StatWidgetComponent`))))
  (set `self.StatUI` _aswb_lobby_field_player_stat_ui)
  (`self.PlayerMeshSelect`)
  (`TextBlock.SetText` (`/Game/StrangeShowdown/UI/Interfaces/WB_LobbyFieldPlayerStatUI.Nickname` (`self.StatUI`)) (`KismetTextLibrary.Conv_StringToText` (`self.PlayerNickName`))))

(fn `PlayerMeshSelect`
  (switch `EPlayerMeshType` (`self.PlayerMeshType`)
    (:`Badguy`
      (`SkeletalMeshComponent.SetSkeletalMeshAsset` (`self.Mesh`) "/Game/PolygonWestern/Meshes/CharactersUE4Mannequin/SK_Chr_Badguy_01.SK_Chr_Badguy_01"))
    (:`BuisinessMan`
      (`SkeletalMeshComponent.SetSkeletalMeshAsset` (`self.Mesh`) "/Game/PolygonWestern/Meshes/CharactersUE4Mannequin/SK_Chr_Business_Man_01.SK_Chr_Business_Man_01"))
    (:`Cowboy`
      (`SkeletalMeshComponent.SetSkeletalMeshAsset` (`self.Mesh`) "/Game/PolygonWestern/Meshes/CharactersUE4Mannequin/SK_Chr_Cowboy_01.SK_Chr_Cowboy_01"))
    (:`Cowgirl`
      (`SkeletalMeshComponent.SetSkeletalMeshAsset` (`self.Mesh`) "/Game/PolygonWestern/Meshes/CharactersUE4Mannequin/SK_Chr_Cowgirl_01.SK_Chr_Cowgirl_01"))
    (:`Gunman`
      (`SkeletalMeshComponent.SetSkeletalMeshAsset` (`self.Mesh`) "/Game/PolygonWestern/Meshes/CharactersUE4Mannequin/SK_Chr_Gunman_01.SK_Chr_Gunman_01"))
    (:`Woman`
      (`SkeletalMeshComponent.SetSkeletalMeshAsset` (`self.Mesh`) "/Game/PolygonWestern/Meshes/CharactersUE4Mannequin/SK_Chr_Woman_01.SK_Chr_Woman_01"))
    (:`WorkingGirl`
      (`SkeletalMeshComponent.SetSkeletalMeshAsset` (`self.Mesh`) "/Game/PolygonWestern/Meshes/CharactersUE4Mannequin/SK_Chr_WorkingGirl_01.SK_Chr_WorkingGirl_01"))))

(fn `UserConstructionScript`)