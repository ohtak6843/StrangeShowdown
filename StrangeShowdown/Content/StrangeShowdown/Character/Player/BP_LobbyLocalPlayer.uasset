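; Lobby pawn for the local player, showing the character mesh that matches its selected player type.
; On BeginPlay it caches the lobby controller, then PlayerMeshSelect maps the PlayerMeshType enum to one of the Western-style skeletal meshes.
; Debug keys spawn temporary field players at fixed spots into FieldPlayers, or destroy the first one found in the world without removing it from that array.
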(event EventBeginPlay
  ;[0.15 0.15 0.15 0.5] BeginPlay
  (bind _aspc_lobby_controller (Utilities|Casting|CastToPC_LobbyController (Pawn|GetController)))
  (Variables|Default|SetPlayerController _aspc_lobby_controller)
  (CallFunction|PlayerMeshSelect))

(event Input|KeyboardEvents|DebugKey2
  (params (Key :type Key%20Structure :default "None") (ActionValue :type Input%20Action%20Value%20Structure))
  (:Pressed
    (bind _outactors (Actor|GetAllActorsOfClass "/Game/StrangeShowdown/Character/Player/BP_LobbyFieldPlayerTemp.BP_LobbyFieldPlayerTemp_C"))
    (Actor|DestroyActor (Utilities|Array|Get(acopy) _outactors))))

(event Input|KeyboardEvents|DebugKey1
  (params (Key :type Key%20Structure :default "None") (ActionValue :type Input%20Action%20Value%20Structure))
  (:Pressed
    (bind _returnvalue (Game|SpawnActorfromClass "/Game/StrangeShowdown/Character/Player/BP_LobbyFieldPlayerTemp.BP_LobbyFieldPlayerTemp_C" (Math|Transform|MakeTransform "-909.545778,22.554325,134.413740" "0, 0, 0" "1.000000,1.000000,1.000000") "Undefined" "MultiplyWithRoot" 0 0))
    (Utilities|Array|Add (Variables|Default|GetFieldPlayers) _returnvalue)))

(event Input|KeyboardEvents|DebugKey3
  (params (Key :type Key%20Structure :default "None") (ActionValue :type Input%20Action%20Value%20Structure))
  (:Pressed
    (bind _returnvalue (Game|SpawnActorfromClass "/Game/StrangeShowdown/Character/Player/BP_LobbyFieldPlayerTemp.BP_LobbyFieldPlayerTemp_C" (Math|Transform|MakeTransform "-909.545778,22.554325,1000.000000" "0, 0, 0" "1.000000,1.000000,1.000000") "Undefined" "MultiplyWithRoot" 0 0))
    (Utilities|Array|Add (Variables|Default|GetFieldPlayers) _returnvalue)))

(fn ConstructionScript)

(fn PlayerMeshSelect
  (switch Utilities|FlowControl|Switch|SwitchonEPlayerMeshType (Variables|Default|GetPlayerMeshType)
    (:Badguy
      (Components|SkeletalMesh|SetSkeletalMeshAsset (Variables|Character|GetMesh) "/Game/PolygonWestern/Meshes/CharactersUE4Mannequin/SK_Chr_Badguy_01.SK_Chr_Badguy_01"))
    (:BuisinessMan
      (Components|SkeletalMesh|SetSkeletalMeshAsset (Variables|Character|GetMesh) "/Game/PolygonWestern/Meshes/CharactersUE4Mannequin/SK_Chr_Business_Man_01.SK_Chr_Business_Man_01"))
    (:Cowboy
      (Components|SkeletalMesh|SetSkeletalMeshAsset (Variables|Character|GetMesh) "/Game/PolygonWestern/Meshes/CharactersUE4Mannequin/SK_Chr_Cowboy_01.SK_Chr_Cowboy_01"))
    (:Cowgirl
      (Components|SkeletalMesh|SetSkeletalMeshAsset (Variables|Character|GetMesh) "/Game/PolygonWestern/Meshes/CharactersUE4Mannequin/SK_Chr_Cowgirl_01.SK_Chr_Cowgirl_01"))
    (:Gunman
      (Components|SkeletalMesh|SetSkeletalMeshAsset (Variables|Character|GetMesh) "/Game/PolygonWestern/Meshes/CharactersUE4Mannequin/SK_Chr_Gunman_01.SK_Chr_Gunman_01"))
    (:Woman
      (Components|SkeletalMesh|SetSkeletalMeshAsset (Variables|Character|GetMesh) "/Game/PolygonWestern/Meshes/CharactersUE4Mannequin/SK_Chr_Woman_01.SK_Chr_Woman_01"))
    (:WorkingGirl
      (Components|SkeletalMesh|SetSkeletalMeshAsset (Variables|Character|GetMesh) "/Game/PolygonWestern/Meshes/CharactersUE4Mannequin/SK_Chr_WorkingGirl_01.SK_Chr_WorkingGirl_01"))))