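; Test local player character for Strange Showdown, with working Enhanced Input look and movement.
; BeginPlay adds the input mapping, picks a skeletal mesh from PlayerMeshType and sets the attack trace widget class.
; Pickup, quick slot, aim, fire, store and stat UI events are empty; their former logic is disconnected.
; Functions for pistol fire, sword smash, item use and stat refresh remain, reached only from that disconnected logic.
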(event Custom|InitializeStatUI
  ;[0.15 0.15 0.15 0.5] Stat UI
)

(event Custom|UpdateStatUI
  ;[0.15 0.15 0.15 0.5] Stat UI
)

(event Custom|UpdateStore
  ;[0.15 0.15 0.15 0.5] Store
)

(event Input|EnhancedActionEvents|EnhancedInputActionIA_LookAround
  (params (ActionValue :type Vector%202D%20Structure) (ElapsedSeconds :type Float%20%28double-precision%29) (TriggeredSeconds :type Float%20%28double-precision%29) (InputAction :type Input%20Action%20Object%20Reference :default "/Game/StrangeShowdown/Input/Actions/IA_LookAround.IA_LookAround"))
  ;[0.15 0.15 0.15 0.5] IA_LookAround
  (Pawn|Input|AddControllerYawInput (.x ActionValue))
  (Pawn|Input|AddControllerPitchInput (* (.y ActionValue) -1.0)))

(event Input|EnhancedActionEvents|EnhancedInputActionIA_Movement
  (params (ActionValue :type Vector%202D%20Structure) (ElapsedSeconds :type Float%20%28double-precision%29) (TriggeredSeconds :type Float%20%28double-precision%29) (InputAction :type Input%20Action%20Object%20Reference :default "/Game/StrangeShowdown/Input/Actions/IA_Movement.IA_Movement"))
  (bind _returnvalue (Pawn|GetControlRotation :!class /Script/Engine.Pawn))
  ;[0.15 0.15 0.15 0.5] IA_Movement
  (Pawn|Input|AddMovementInput (Math|Vector|GetRightVector (Math|Rotator|MakeRotator (.roll _returnvalue) 0.0 (.yaw _returnvalue))) (.x ActionValue) false)
  (Pawn|Input|AddMovementInput (Math|Vector|GetForwardVector (Math|Rotator|MakeRotator 0.0 0.0 (.yaw (Pawn|GetControlRotation :!class /Script/Engine.Pawn)))) (.y ActionValue) false))

(event Input|EnhancedActionEvents|EnhancedInputActionIA_QuickSlot2
  (params (ActionValue :type Boolean) (ElapsedSeconds :type Float%20%28double-precision%29) (TriggeredSeconds :type Float%20%28double-precision%29) (InputAction :type Input%20Action%20Object%20Reference :default "/Game/StrangeShowdown/Input/Actions/IA_QuickSlot2.IA_QuickSlot2"))
  ;[0.15 0.15 0.15 0.5] IA_QuickSlots
)

(event Input|EnhancedActionEvents|EnhancedInputActionIA_QuickSlot3
  (params (ActionValue :type Boolean) (ElapsedSeconds :type Float%20%28double-precision%29) (TriggeredSeconds :type Float%20%28double-precision%29) (InputAction :type Input%20Action%20Object%20Reference :default "/Game/StrangeShowdown/Input/Actions/IA_QuickSlot3.IA_QuickSlot3"))
  ;[0.15 0.15 0.15 0.5] IA_QuickSlots
)

(event Input|EnhancedActionEvents|EnhancedInputActionIA_QuickSlot4
  (params (ActionValue :type Boolean) (ElapsedSeconds :type Float%20%28double-precision%29) (TriggeredSeconds :type Float%20%28double-precision%29) (InputAction :type Input%20Action%20Object%20Reference :default "/Game/StrangeShowdown/Input/Actions/IA_QuickSlot4.IA_QuickSlot4"))
  ;[0.15 0.15 0.15 0.5] IA_QuickSlots
)

(event Input|EnhancedActionEvents|EnhancedInputActionIA_QuickSlot5
  (params (ActionValue :type Boolean) (ElapsedSeconds :type Float%20%28double-precision%29) (TriggeredSeconds :type Float%20%28double-precision%29) (InputAction :type Input%20Action%20Object%20Reference :default "/Game/StrangeShowdown/Input/Actions/IA_QuickSlot5.IA_QuickSlot5"))
  ;[0.15 0.15 0.15 0.5] IA_QuickSlots
)

(event Input|EnhancedActionEvents|EnhancedInputActionIA_Pickup
  (params (ActionValue :type Boolean) (ElapsedSeconds :type Float%20%28double-precision%29) (TriggeredSeconds :type Float%20%28double-precision%29) (InputAction :type Input%20Action%20Object%20Reference :default "/Game/StrangeShowdown/Input/Actions/IA_Pickup.IA_Pickup"))
  ;[0.15 0.15 0.15 0.5] IA_Pickup
)

(event Input|EnhancedActionEvents|EnhancedInputActionIA_PistolAim
  (params (ActionValue :type Boolean) (ElapsedSeconds :type Float%20%28double-precision%29) (TriggeredSeconds :type Float%20%28double-precision%29) (InputAction :type Input%20Action%20Object%20Reference :default "/Game/StrangeShowdown/Input/Actions/IA_PistolAim.IA_PistolAim"))
  ;[0.15 0.15 0.15 0.5] IA_Aiming
)

(event Input|EnhancedActionEvents|EnhancedInputActionIA_QuickSlot1
  (params (ActionValue :type Boolean) (ElapsedSeconds :type Float%20%28double-precision%29) (TriggeredSeconds :type Float%20%28double-precision%29) (InputAction :type Input%20Action%20Object%20Reference :default "/Game/StrangeShowdown/Input/Actions/IA_QuickSlot1.IA_QuickSlot1"))
  ;[0.15 0.15 0.15 0.5] IA_QuickSlots
)

(event Input|EnhancedActionEvents|EnhancedInputActionIA_PistolFire
  (params (ActionValue :type Boolean) (ElapsedSeconds :type Float%20%28double-precision%29) (TriggeredSeconds :type Float%20%28double-precision%29) (InputAction :type Input%20Action%20Object%20Reference :default "/Game/StrangeShowdown/Input/Actions/IA_PistolFire.IA_PistolFire"))
  ;[0.15 0.15 0.15 0.5] IA_GunFire
)

(event Input|EnhancedActionEvents|EnhancedInputActionIA_QuickSlot6
  (params (ActionValue :type Boolean) (ElapsedSeconds :type Float%20%28double-precision%29) (TriggeredSeconds :type Float%20%28double-precision%29) (InputAction :type Input%20Action%20Object%20Reference :default "/Game/StrangeShowdown/Input/Actions/IA_QuickSlot6.IA_QuickSlot6"))
  ;[0.15 0.15 0.15 0.5] IA_QuickSlots
)

(event Input|EnhancedActionEvents|EnhancedInputActionIA_QuickSlotScroll
  (params (ActionValue :type Float%20%28double-precision%29) (ElapsedSeconds :type Float%20%28double-precision%29) (TriggeredSeconds :type Float%20%28double-precision%29) (InputAction :type Input%20Action%20Object%20Reference :default "/Game/StrangeShowdown/Input/Actions/IA_QuickSlotScroll.IA_QuickSlotScroll"))
  ;[0.15 0.15 0.15 0.5] IA_QuickSlots
)

(event EventBeginPlay
  ;[0.15 0.15 0.15 0.5] BeginPlay
  (bind _asplayer_controller (Utilities|Casting|CastToPlayerController (Pawn|GetController)))
  (Input|AddMappingContext (PlayerController|LocalPlayerSubsystems|GetEnhancedInputLocalPlayerSubsystem _asplayer_controller) "/Game/StrangeShowdown/Input/IMC_PlayerInput.IMC_PlayerInput" 0 "(bIgnoreAllPressedKeysUntilRelease=True,bForceImmediately=False,bNotifyUserSettings=False)")
  (CallFunction|PlayerMeshSelect)
  (Variables|/Script/StrangeShowdown.STAttackTraceComponent|SetAttackTraceWidgetClass (Variables|Default|GetAttackTraceComp) "/Game/StrangeShowdown/UI/AttackTrace/WB_AttackTrace.WB_AttackTrace_C"))

(event Input|KeyboardEvents|DebugKey9
  (params (Key :type Key%20Structure :default "None") (ActionValue :type Input%20Action%20Value%20Structure))
  ;[0.15 0.15 0.15 0.5] Debug Key
)

(event Input|KeyboardEvents|DebugKey0
  (params (Key :type Key%20Structure :default "None") (ActionValue :type Input%20Action%20Value%20Structure))
  ;[0.15 0.15 0.15 0.5] Debug Key
)

(event Input|KeyboardEvents|DebugKeyR
  (params (Key :type Key%20Structure :default "None") (ActionValue :type Input%20Action%20Value%20Structure))
  ;[0.15 0.15 0.15 0.5] Debug Key
)

(fn ConstructionScript)

(fn UpdateAllStat
  (bind _statcomp (Variables|Default|GetStatComp))
  (bind _aswb_stat (Utilities|Casting|CastToWB_Stat (Variables|/Script/StrangeShowdown.STHUD|GetStatWidget (Variables|/Game/StrangeShowdown/Controller/PC_PlayerController.PC_PlayerController_C|GetPlayer%20HUD (Variables|Default|GetPlayerController)))))
  (Default|UpdateActionUI _aswb_stat _statcomp)
  (Default|UpdateGoldUI _aswb_stat _statcomp)
  (Default|UpdateStaminaUI _aswb_stat _statcomp)
  (Default|UpdateHpUI _aswb_stat _statcomp)
  (Default|UpdateHelmetUI _aswb_stat _statcomp))

(fn PlayerMeshSelect
  (switch Utilities|FlowControl|Switch|SwitchonEPlayerMeshType (Variables|Default|GetPlayerMeshType)
    (:Badguy
      (Components|SkeletalMesh|SetSkeletalMeshAsset (Variables|Character|GetMesh) "/Game/PolygonWestern/Meshes/CharactersUE4Mannequin/SK_Chr_Badguy_01.SK_Chr_Badguy_01"))
    (:BuisinessMan
      (Components|SkeletalMesh|SetSkeletalMeshAsset (Variables|Character|GetMesh) "/Game/PolygonWestern/Meshes/CharactersUE4Mannequin/SK_Chr_Business_Man_01.SK_Chr_Business_Man_01"))
    (:Cowboy
      (Components|SkeletalMesh|SetSkeletalMeshAsset (Variables|Character|GetMesh) "/Game/PolygonWestern/Meshes/CharactersUE4Mannequin/SK_Chr_Cowboy_01.SK_Chr_Cowboy_01"))
    (:Cowgirl
      (Components|SkeletalMesh|SetSkeletalMeshAsset (Variables|Character|GetMesh) "/Game/PolygonWestern/Meshes/CharactersUE4Mannequin/SK_Chr_Cowgirl_01.SK_Chr_Cowgirl_01"))
    (:Gunman
      (Components|SkeletalMesh|SetSkeletalMeshAsset (Variables|Character|GetMesh) "/Game/PolygonWestern/Meshes/CharactersUE4Mannequin/SK_Chr_Gunman_01.SK_Chr_Gunman_01"))
    (:Woman
      (Components|SkeletalMesh|SetSkeletalMeshAsset (Variables|Character|GetMesh) "/Game/PolygonWestern/Meshes/CharactersUE4Mannequin/SK_Chr_Woman_01.SK_Chr_Woman_01"))
    (:WorkingGirl
      (Components|SkeletalMesh|SetSkeletalMeshAsset (Variables|Character|GetMesh) "/Game/PolygonWestern/Meshes/CharactersUE4Mannequin/SK_Chr_WorkingGirl_01.SK_Chr_WorkingGirl_01"))))

(fn PlayMuzzleFlash
  (bind _righthandskeletalmesh (Variables|Default|GetRightHandSkeletalMesh))
  (Niagara|SpawnSystematLocation "/Game/StrangeShowdown/Item/FX/NS_PistolMuzzleFlash.NS_PistolMuzzleFlash" (Transformation|GetSocketLocation _righthandskeletalmesh "Muzzle") (Transformation|GetSocketRotation _righthandskeletalmesh "Muzzle")))

(fn Fire
  (Game|Damage|ApplyDamage (Variables|/Script/StrangeShowdown.STAttackTraceComponent|GetTracingFieldPlayer (Variables|Default|GetAttackTraceComp)) 1.0 0 self)
  (bind _asbp_field_player (Utilities|Casting|CastToBP_FieldPlayer (Variables|/Script/StrangeShowdown.STAttackTraceComponent|GetTracingFieldPlayer (Variables|Default|GetAttackTraceComp))))
  (Default|UpdateAllStat _asbp_field_player)
  (CallFunction|PlayMuzzleFlash)
  (Camera|PlayWorldCameraShake "/Game/StrangeShowdown/CameraShake/BP_CameraShake.BP_CameraShake_C" (Transformation|GetActorLocation) 0.0 5e+02)
  (Audio|SpawnSound2D "/Game/StrangeShowdown/Sound/Effect/SW_Fire.SW_Fire" 1.0 1.0 0.0 0))

(fn UseItem
  (bind (_outslot _returnvalue) (Class|STInventoryComponent|UseItem (Variables|Default|GetInventoryComp) (Utilities|Array|Get(acopy) (Variables|/Script/StrangeShowdown.STQuickSlotComponent|GetInventorySlotIndex (Variables|Default|GetQuickSlotComp)) (Variables|Default|GetCurrentSelectQuickSlotIndex)) self))
  (switch Utilities|FlowControl|Switch|SwitchonEItemUseType _returnvalue
    (:CanUse
      (bind _returnvalue_2 (UserInterface|CreateWidget "/Game/StrangeShowdown/UI/WB_FloatingMessage.WB_FloatingMessage_C"))
      (UserInterface|Viewport|AddtoViewport _returnvalue_2 100)
      (Rendering|Components|TextRender|SetText (Variables|/Game/StrangeShowdown/UI/WB_FloatingMessage.WB_FloatingMessage_C|GetMessage _returnvalue_2) (Variables|/Script/StrangeShowdown.STItemDataAssetBase|GetItemName (.ItemData (Utilities|Struct|BreakSTItemSlot _outslot))))
      (Class|STLocalPlayer|HoldItem))
    (:NotEnoughStaminaCost
      (CallFunction|NotEnoughStaminaCostFloatingMessage))
    (:Exception
      (bind _returnvalue_3 (UserInterface|CreateWidget "/Game/StrangeShowdown/UI/WB_FloatingMessage.WB_FloatingMessage_C"))
      (UserInterface|Viewport|AddtoViewport _returnvalue_3 100)
      (Rendering|Components|TextRender|SetText (Variables|/Game/StrangeShowdown/UI/WB_FloatingMessage.WB_FloatingMessage_C|GetMessage _returnvalue_3) "배고파?")
      (Audio|SpawnSound2D "/Game/StrangeShowdown/Sound/Effect/SW_Error.SW_Error" 0.8 1.0 0.0 0))))

(fn Smash
  (Variables|Default|SetIsSmashing true)
  (Animation|PlayAnimMontage "/Game/PolygonWestern/EpicContent/Mannequin/RetargetAnimations/Hammer/Great_Sword_Slash_Montage.Great_Sword_Slash_Montage" 1.0 "None"))

(fn NotEnoughStaminaCostFloatingMessage
  (bind _returnvalue (UserInterface|CreateWidget "/Game/StrangeShowdown/UI/WB_FloatingMessage.WB_FloatingMessage_C"))
  (UserInterface|Viewport|AddtoViewport _returnvalue 100)
  (Rendering|Components|TextRender|SetText (Variables|/Game/StrangeShowdown/UI/WB_FloatingMessage.WB_FloatingMessage_C|GetMessage _returnvalue) "스태미너 부족!")
  (Audio|SpawnSound2D "/Game/StrangeShowdown/Sound/Effect/SW_Error.SW_Error" 0.8 1.0 0.0 0))