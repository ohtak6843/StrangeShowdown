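; BP_LocalPlayerBase is the locally controlled player character, handling input, character mesh selection and HUD updates.
; BeginPlay sets up input, quick slots, stat UI, mesh and a placeholder store item.
; Quick-slot selection drives the primary action: slot one fires at the AttackTraceComp target while aiming, slot two is a stub smash, others use inventory items.
; Pickups feed inventory and quick slots; debug keys test stats, door slicing and missions.
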(event Custom|UpdateInventory
  (bind _playercontroller (Variables|Default|GetPlayerController))
  (bind _player_hud (Variables|/Game/StrangeShowdown/Controller/PC_PlayerController.PC_PlayerController_C|GetPlayer%20HUD _playercontroller))
  (bind _wb_inventorymenu (Variables|/Game/StrangeShowdown/UI/WB_HUD.WB_HUD_C|GetWB_InventoryMenu _player_hud))
  ;[0.15 0.15 0.15 0.5] Inventory
  (Utilities|IsValid _wb_inventorymenu
    (:Is%20Valid
      (Default|UpdateInventory (Variables|/Game/StrangeShowdown/UI/Inventory/WB_InventoryMenu.WB_InventoryMenu_C|GetWB_Inventory _wb_inventorymenu) (Variables|Default|GetInventoryComp)))))

(event Custom|InitializeQuickSlot
  ;[0.15 0.15 0.15 0.5] Inventory
  (Default|InitializeQuickSlot (Variables|/Game/StrangeShowdown/Controller/PC_PlayerController.PC_PlayerController_C|GetPlayer%20HUD (Variables|Default|GetPlayerController)) (Variables|Default|GetQuickSlotComp)))

(event Custom|InitializeStatUI
  (bind _playercontroller (Variables|Default|GetPlayerController))
  (bind _player_hud (Variables|/Game/StrangeShowdown/Controller/PC_PlayerController.PC_PlayerController_C|GetPlayer%20HUD _playercontroller))
  (bind _wb_tabuimenu (Variables|/Game/StrangeShowdown/UI/WB_HUD.WB_HUD_C|GetWB_TabUIMenu _player_hud))
  ;[0.15 0.15 0.15 0.5] Stat UI
  (CallFunction|UpdateAllStat) ; 자신의 UI
  (Utilities|IsValid _wb_tabuimenu
    (:Is%20Valid
      (Default|UpdateTabUI (Variables|/Game/StrangeShowdown/UI/TabUI/WB_TabUIMenu.WB_TabUIMenu_C|GetWB_TabUI _wb_tabuimenu)) ; Update Stat UI 이벤트가 호출되면\nTab UI도 새로 만들어 업데이트를 처리함
    )))

(event Custom|UpdateStatUI
  (bind _playercontroller (Variables|Default|GetPlayerController))
  (bind _player_hud (Variables|/Game/StrangeShowdown/Controller/PC_PlayerController.PC_PlayerController_C|GetPlayer%20HUD _playercontroller))
  (bind _wb_tabuimenu (Variables|/Game/StrangeShowdown/UI/WB_HUD.WB_HUD_C|GetWB_TabUIMenu _player_hud))
  ;[0.15 0.15 0.15 0.5] Stat UI
  (CallFunction|UpdateAllStat) ; 자신의 UI
  (Utilities|IsValid _wb_tabuimenu
    (:Is%20Valid
      (Default|UpdateTabUI (Variables|/Game/StrangeShowdown/UI/TabUI/WB_TabUIMenu.WB_TabUIMenu_C|GetWB_TabUI _wb_tabuimenu)) ; Update Stat UI 이벤트가 호출되면\nTab UI도 새로 만들어 업데이트를 처리함
    )))

(event Custom|UpdateStore
  (bind _playercontroller (Variables|Default|GetPlayerController))
  (bind _player_hud (Variables|/Game/StrangeShowdown/Controller/PC_PlayerController.PC_PlayerController_C|GetPlayer%20HUD _playercontroller))
  (bind _wb_storemenu (Variables|/Game/StrangeShowdown/UI/WB_HUD.WB_HUD_C|GetWB_StoreMenu _player_hud))
  ;[0.15 0.15 0.15 0.5] Store
  (Utilities|IsValid _wb_storemenu
    (:Is%20Valid
      (Default|UpdateStore (Variables|/Game/StrangeShowdown/UI/Store/WB_StoreMenu.WB_StoreMenu_C|GetWB_Store _wb_storemenu) (Variables|Default|GetStoreComp)))))

(event Input|EnhancedActionEvents|EnhancedInputActionIA_LookAround
  (params (ActionValue :type Vector%202D%20Structure) (ElapsedSeconds :type Float%20%28double-precision%29) (TriggeredSeconds :type Float%20%28double-precision%29) (InputAction :type Input%20Action%20Object%20Reference :default "/Game/StrangeShowdown/Input/Actions/IA_LookAround.IA_LookAround"))
  ;[0.15 0.15 0.15 0.5] IA_LookAround
  (Pawn|Input|AddControllerYawInput (.x ActionValue))
  (Pawn|Input|AddControllerPitchInput (* (.y ActionValue) -1.0)))

(event Input|EnhancedActionEvents|EnhancedInputActionIA_Movement
  (params (ActionValue :type Vector%202D%20Structure) (ElapsedSeconds :type Float%20%28double-precision%29) (TriggeredSeconds :type Float%20%28double-precision%29) (InputAction :type Input%20Action%20Object%20Reference :default "/Game/StrangeShowdown/Input/Actions/IA_Movement.IA_Movement"))
  (bind _returnvalue (Pawn|GetControlRotation :!class /Script/Engine.Pawn))
  ;[0.15 0.15 0.15 0.5] IA_Movement
  (Pawn|Input|AddMovementInput (Math|Vector|GetRightVector (Math|Rotator|MakeRotator (.roll _returnvalue) 0.0 (.yaw _returnvalue))) (.x ActionValue) false)
  (Pawn|Input|AddMovementInput (Math|Vector|GetForwardVector (Math|Rotator|MakeRotator 0.0 0.0 (.yaw (Pawn|GetControlRotation :!class /Script/Engine.Pawn)))) (.y ActionValue) false))

(event Input|EnhancedActionEvents|EnhancedInputActionIA_QuickSlot2
  (params (ActionValue :type Boolean) (ElapsedSeconds :type Float%20%28double-precision%29) (TriggeredSeconds :type Float%20%28double-precision%29) (InputAction :type Input%20Action%20Object%20Reference :default "/Game/StrangeShowdown/Input/Actions/IA_QuickSlot2.IA_QuickSlot2"))
  ;[0.15 0.15 0.15 0.5] IA_QuickSlots
  (:Started
    (bind _output_get (Variables|Default|SetCurrentSelectQuickSlotIndex 1))
    (Variables|/Script/StrangeShowdown.STQuickSlotComponent|SetCurrentSelectQuickSlotIndex (Variables|Default|GetQuickSlotComp) _output_get)
    (if (Class|STPlayerBase|HasAllStateMask 32)
      (Class|STLocalPlayer|ApplyStateSettings "Idle"))
    (Default|UpdateQuickSlotfromUseItem (Variables|/Game/StrangeShowdown/Controller/PC_PlayerController.PC_PlayerController_C|GetPlayer%20HUD (Variables|Default|GetPlayerController)) (Variables|Default|GetQuickSlotComp))
    (Class|STLocalPlayer|HoldItem)))

(event Input|EnhancedActionEvents|EnhancedInputActionIA_QuickSlot3
  (params (ActionValue :type Boolean) (ElapsedSeconds :type Float%20%28double-precision%29) (TriggeredSeconds :type Float%20%28double-precision%29) (InputAction :type Input%20Action%20Object%20Reference :default "/Game/StrangeShowdown/Input/Actions/IA_QuickSlot3.IA_QuickSlot3"))
  ;[0.15 0.15 0.15 0.5] IA_QuickSlots
  (:Started
    (bind _output_get (Variables|Default|SetCurrentSelectQuickSlotIndex 2))
    (Variables|/Script/StrangeShowdown.STQuickSlotComponent|SetCurrentSelectQuickSlotIndex (Variables|Default|GetQuickSlotComp) _output_get)
    (if (Class|STPlayerBase|HasAllStateMask 32)
      (Class|STLocalPlayer|ApplyStateSettings "Idle"))
    (Default|UpdateQuickSlotfromUseItem (Variables|/Game/StrangeShowdown/Controller/PC_PlayerController.PC_PlayerController_C|GetPlayer%20HUD (Variables|Default|GetPlayerController)) (Variables|Default|GetQuickSlotComp))
    (Class|STLocalPlayer|HoldItem)))

(event Input|EnhancedActionEvents|EnhancedInputActionIA_QuickSlot4
  (params (ActionValue :type Boolean) (ElapsedSeconds :type Float%20%28double-precision%29) (TriggeredSeconds :type Float%20%28double-precision%29) (InputAction :type Input%20Action%20Object%20Reference :default "/Game/StrangeShowdown/Input/Actions/IA_QuickSlot4.IA_QuickSlot4"))
  ;[0.15 0.15 0.15 0.5] IA_QuickSlots
  (:Started
    (bind _output_get (Variables|Default|SetCurrentSelectQuickSlotIndex 3))
    (Variables|/Script/StrangeShowdown.STQuickSlotComponent|SetCurrentSelectQuickSlotIndex (Variables|Default|GetQuickSlotComp) _output_get)
    (if (Class|STPlayerBase|HasAllStateMask 32)
      (Class|STLocalPlayer|ApplyStateSettings "Idle"))
    (Default|UpdateQuickSlotfromUseItem (Variables|/Game/StrangeShowdown/Controller/PC_PlayerController.PC_PlayerController_C|GetPlayer%20HUD (Variables|Default|GetPlayerController)) (Variables|Default|GetQuickSlotComp))
    (Class|STLocalPlayer|HoldItem)))

(event Input|EnhancedActionEvents|EnhancedInputActionIA_QuickSlot5
  (params (ActionValue :type Boolean) (ElapsedSeconds :type Float%20%28double-precision%29) (TriggeredSeconds :type Float%20%28double-precision%29) (InputAction :type Input%20Action%20Object%20Reference :default "/Game/StrangeShowdown/Input/Actions/IA_QuickSlot5.IA_QuickSlot5"))
  ;[0.15 0.15 0.15 0.5] IA_QuickSlots
  (:Started
    (bind _output_get (Variables|Default|SetCurrentSelectQuickSlotIndex 4))
    (Variables|/Script/StrangeShowdown.STQuickSlotComponent|SetCurrentSelectQuickSlotIndex (Variables|Default|GetQuickSlotComp) _output_get)
    (if (Class|STPlayerBase|HasAllStateMask 32)
      (Class|STLocalPlayer|ApplyStateSettings "Idle"))
    (Default|UpdateQuickSlotfromUseItem (Variables|/Game/StrangeShowdown/Controller/PC_PlayerController.PC_PlayerController_C|GetPlayer%20HUD (Variables|Default|GetPlayerController)) (Variables|Default|GetQuickSlotComp))
    (Class|STLocalPlayer|HoldItem)))

(event Input|EnhancedActionEvents|EnhancedInputActionIA_Pickup
  (params (ActionValue :type Boolean) (ElapsedSeconds :type Float%20%28double-precision%29) (TriggeredSeconds :type Float%20%28double-precision%29) (InputAction :type Input%20Action%20Object%20Reference :default "/Game/StrangeShowdown/Input/Actions/IA_Pickup.IA_Pickup"))
  ;[0.15 0.15 0.15 0.5] IA_Pickup
  (:Started
    (bind _outaddedinventoryindex (Class|STLocalPlayer|Interact))
    (CallFunction|UpdateInventory)
    (Class|STQuickSlotComponent|AddtoQuickSlot (Variables|Default|GetQuickSlotComp) (Variables|Default|GetInventoryComp) _outaddedinventoryindex -2) ; -2면 즉시 추가
    (Default|UpdateQuickSlot (Variables|/Game/StrangeShowdown/Controller/PC_PlayerController.PC_PlayerController_C|GetPlayer%20HUD (Variables|Default|GetPlayerController)))
    (Class|STLocalPlayer|HoldItem)))

(event Input|EnhancedActionEvents|EnhancedInputActionIA_GunAiming
  (params (ActionValue :type Boolean) (ElapsedSeconds :type Float%20%28double-precision%29) (TriggeredSeconds :type Float%20%28double-precision%29) (InputAction :type Input%20Action%20Object%20Reference :default "/Game/StrangeShowdown/Input/Actions/IA_GunAiming.IA_GunAiming"))
  ;[0.15 0.15 0.15 0.5] IA_Aiming
  (if (Class|STPlayerBase|HasAnyStateMask 32)
    (Class|STLocalPlayer|ApplyStateSettings "Idle")
    (else
      (Variables|/Script/StrangeShowdown.STQuickSlotComponent|SetCurrentSelectQuickSlotIndex (Variables|Default|GetQuickSlotComp) 0)
      (Default|UpdateQuickSlotfromUseItem (Variables|/Game/StrangeShowdown/Controller/PC_PlayerController.PC_PlayerController_C|GetPlayer%20HUD (Variables|Default|GetPlayerController)) (Variables|Default|GetQuickSlotComp))
      (Class|STLocalPlayer|ApplyStateSettings "Aiming")
      (Class|STLocalPlayer|HoldItem))))

(event Input|EnhancedActionEvents|EnhancedInputActionIA_QuickSlot1
  (params (ActionValue :type Boolean) (ElapsedSeconds :type Float%20%28double-precision%29) (TriggeredSeconds :type Float%20%28double-precision%29) (InputAction :type Input%20Action%20Object%20Reference :default "/Game/StrangeShowdown/Input/Actions/IA_QuickSlot1.IA_QuickSlot1"))
  ;[0.15 0.15 0.15 0.5] IA_QuickSlots
  (:Started
    (bind _output_get (Variables|Default|SetCurrentSelectQuickSlotIndex 0))
    (Variables|/Script/StrangeShowdown.STQuickSlotComponent|SetCurrentSelectQuickSlotIndex (Variables|Default|GetQuickSlotComp) _output_get)
    (Default|UpdateQuickSlotfromUseItem (Variables|/Game/StrangeShowdown/Controller/PC_PlayerController.PC_PlayerController_C|GetPlayer%20HUD (Variables|Default|GetPlayerController)) (Variables|Default|GetQuickSlotComp))
    (Class|STLocalPlayer|HoldItem)))

(event Input|EnhancedActionEvents|EnhancedInputActionIA_GunFire
  (params (ActionValue :type Boolean) (ElapsedSeconds :type Float%20%28double-precision%29) (TriggeredSeconds :type Float%20%28double-precision%29) (InputAction :type Input%20Action%20Object%20Reference :default "/Game/StrangeShowdown/Input/Actions/IA_GunFire.IA_GunFire"))
  ;[0.15 0.15 0.15 0.5] IA_GunFire
  (:Started
    (if (== (Variables|/Script/StrangeShowdown.STQuickSlotComponent|GetCurrentSelectQuickSlotIndex (Variables|Default|GetQuickSlotComp)) 0)
      (if (Class|STPlayerBase|HasAnyStateMask 32)
        (Utilities|IsValid (Variables|/Script/StrangeShowdown.STAttackTraceComponent|GetTracingFieldPlayer (Variables|Default|GetAttackTraceComp))
          (:Is%20Valid
            (CallFunction|Fire))))
      (elif (== (Variables|/Script/StrangeShowdown.STQuickSlotComponent|GetCurrentSelectQuickSlotIndex (Variables|Default|GetQuickSlotComp)) 1)
        (CallFunction|Smash)
        (else
          (CallFunction|UseItem))))))

(event Input|EnhancedActionEvents|EnhancedInputActionIA_QuickSlot6
  (params (ActionValue :type Boolean) (ElapsedSeconds :type Float%20%28double-precision%29) (TriggeredSeconds :type Float%20%28double-precision%29) (InputAction :type Input%20Action%20Object%20Reference :default "/Game/StrangeShowdown/Input/Actions/IA_QuickSlot6.IA_QuickSlot6"))
  ;[0.15 0.15 0.15 0.5] IA_QuickSlots
  (:Started
    (bind _output_get (Variables|Default|SetCurrentSelectQuickSlotIndex 5))
    (Variables|/Script/StrangeShowdown.STQuickSlotComponent|SetCurrentSelectQuickSlotIndex (Variables|Default|GetQuickSlotComp) _output_get)
    (if (Class|STPlayerBase|HasAllStateMask 32)
      (Class|STLocalPlayer|ApplyStateSettings "Idle"))
    (Default|UpdateQuickSlotfromUseItem (Variables|/Game/StrangeShowdown/Controller/PC_PlayerController.PC_PlayerController_C|GetPlayer%20HUD (Variables|Default|GetPlayerController)) (Variables|Default|GetQuickSlotComp))
    (Class|STLocalPlayer|HoldItem)))

(event Input|EnhancedActionEvents|EnhancedInputActionIA_QuickSlotScroll
  (params (ActionValue :type Float%20%28double-precision%29) (ElapsedSeconds :type Float%20%28double-precision%29) (TriggeredSeconds :type Float%20%28double-precision%29) (InputAction :type Input%20Action%20Object%20Reference :default "/Game/StrangeShowdown/Input/Actions/IA_QuickSlotScroll.IA_QuickSlotScroll"))
  ;[0.15 0.15 0.15 0.5] IA_QuickSlots
  (:Started
    (Math|Float|CompareFloat ActionValue 0.0
      (:>
        (if (>= (+ (Variables|Default|GetCurrentSelectQuickSlotIndex) 1) (Variables|/Script/StrangeShowdown.STQuickSlotComponent|GetQuickSlotSize (Variables|Default|GetQuickSlotComp))) :!label _label
          (bind _output_get (Variables|Default|SetCurrentSelectQuickSlotIndex 0))
          (Variables|/Script/StrangeShowdown.STQuickSlotComponent|SetCurrentSelectQuickSlotIndex (Variables|Default|GetQuickSlotComp) _output_get)
          (else
            (bind _output_get_2 (Variables|Default|SetCurrentSelectQuickSlotIndex (+ (Variables|Default|GetCurrentSelectQuickSlotIndex) 1)))
            (Variables|/Script/StrangeShowdown.STQuickSlotComponent|SetCurrentSelectQuickSlotIndex (Variables|Default|GetQuickSlotComp) _output_get_2))))
      (:==
        (goto _label))
      (:<
        (if (<= (- (Variables|Default|GetCurrentSelectQuickSlotIndex) 1) -1)
          (bind _output_get_3 (Variables|Default|SetCurrentSelectQuickSlotIndex (- (Variables|/Script/StrangeShowdown.STQuickSlotComponent|GetQuickSlotSize (Variables|Default|GetQuickSlotComp)) 1)))
          (Variables|/Script/StrangeShowdown.STQuickSlotComponent|SetCurrentSelectQuickSlotIndex (Variables|Default|GetQuickSlotComp) _output_get_3)
          (else
            (bind _output_get_4 (Variables|Default|SetCurrentSelectQuickSlotIndex (- (Variables|Default|GetCurrentSelectQuickSlotIndex) 1)))
            (Variables|/Script/StrangeShowdown.STQuickSlotComponent|SetCurrentSelectQuickSlotIndex (Variables|Default|GetQuickSlotComp) _output_get_4)))))
    (Default|UpdateQuickSlotfromUseItem (Variables|/Game/StrangeShowdown/Controller/PC_PlayerController.PC_PlayerController_C|GetPlayer%20HUD (Variables|Default|GetPlayerController)) (Variables|Default|GetQuickSlotComp))
    (Class|STLocalPlayer|HoldItem)))

(event EventBeginPlay
  (bind _storecomp (Variables|Default|GetStoreComp))
  ;[0.15 0.15 0.15 0.5] BeginPlay
  (bind _aspc_player_controller (Utilities|Casting|CastToPC_PlayerController (Pawn|GetController)))
  (bind _output_get (Variables|Default|SetPlayerController _aspc_player_controller))
  (Input|AddMappingContext (PlayerController|LocalPlayerSubsystems|GetEnhancedInputLocalPlayerSubsystem _output_get) "/Game/StrangeShowdown/Input/IMC_PlayerBaseInput.IMC_PlayerBaseInput" 0 "(bIgnoreAllPressedKeysUntilRelease=True,bForceImmediately=False,bNotifyUserSettings=False)")
  (CallFunction|InitializeQuickSlot)
  (CallFunction|InitializeStatUI)
  (CallFunction|PlayerMeshSelect)
  (Utilities|Array|SetArrayElem (Variables|/Script/StrangeShowdown.STStoreComponent|GetStoreItemPool _storecomp) 0 "/Game/StrangeShowdown/Item/DataAsset/DA_Meat.DA_Meat") ; 임시용 0번 아이템: HealPack
  (Class|STStoreComponent|InitStore _storecomp)
  (Variables|/Script/StrangeShowdown.STAttackTraceComponent|SetAttackTraceWidgetClass (Variables|Default|GetAttackTraceComp) "/Game/StrangeShowdown/UI/AttackTrace/WB_AttackTrace.WB_AttackTrace_C"))

(event Input|KeyboardEvents|DebugKey9
  (params (Key :type Key%20Structure) (ActionValue :type Input%20Action%20Value%20Structure))
  (bind _statcomp (Variables|Default|GetStatComp))
  ;[0.15 0.15 0.15 0.5] Debug Key
  (:Pressed
    (Class|STStatComponent|AddGold _statcomp 1)
    (Development|PrintString (Utilities|String|Append "Gold: " (Utilities|String|ToString(Integer) (Variables|/Script/StrangeShowdown.STStatComponent|GetGold _statcomp))))
    (CallFunction|UpdateStatUI)))

(event Input|KeyboardEvents|DebugKey0
  (params (Key :type Key%20Structure) (ActionValue :type Input%20Action%20Value%20Structure))
  (bind _statcomp (Variables|Default|GetStatComp))
  ;[0.15 0.15 0.15 0.5] Debug Key
  (:Pressed
    (Class|STStatComponent|AddStamina _statcomp 1)
    (Development|PrintString (Utilities|String|Append "Stamina: " (Utilities|String|ToString(Float) (Variables|/Script/StrangeShowdown.STStatComponent|GetCurrentStamina _statcomp))))
    (CallFunction|UpdateStatUI)))

(event Input|KeyboardEvents|DebugKeyQ
  (params (Key :type Key%20Structure) (ActionValue :type Input%20Action%20Value%20Structure))
  (bind _cameracomp (Variables|Default|GetCameraComp))
  (bind _returnvalue (Transformation|GetWorldLocation _cameracomp))
  ;[0.15 0.15 0.15 0.5] Debug(SliceDoor)
  (:Pressed
    (bind _outhit (Collision|LineTraceByChannel _returnvalue (+ _returnvalue (* (Math|Vector|GetForwardVector _cameracomp) 2e+03)) "TraceTypeQuery1" false 0 "ForDuration"))
    (bind _asbp_sliceable_door (Utilities|Casting|CastToBP_SliceableDoor (.HitActor (Collision|BreakHitResult _outhit))))
    (Class|STSliceableActor|Slice _asbp_sliceable_door (.Location (Collision|BreakHitResult _outhit)) (.Normal (Collision|BreakHitResult _outhit)))))

(event Input|KeyboardEvents|DebugKeyR
  (params (Key :type Key%20Structure) (ActionValue :type Input%20Action%20Value%20Structure))
  (:Pressed
    (bind _asstplayer_state (Utilities|Casting|CastToSTPlayerState (Game|GetPlayerState 0)))
    (Class|STMissionComponent|SetMission (Variables|/Script/StrangeShowdown.STPlayerState|GetMissionComponent _asstplayer_state) (Utilities|Text|ToText(String) (Utilities|String|MakeLiteralString "테스트 미션")) (Utilities|Text|ToText(String) (Utilities|String|MakeLiteralString "이 미션은 테스트 미션입니다. 한번 더 말씀 드립니다. 테스트 미션입니다.")))))

(fn ConstructionScript)

(fn UpdateAllStat
  (bind _statcomp (Variables|Default|GetStatComp))
  (bind _aswb_stat (Utilities|Casting|CastToWB_Stat (Variables|/Script/StrangeShowdown.STHUD|GetStatWidget (Variables|/Game/StrangeShowdown/Controller/PC_PlayerController.PC_PlayerController_C|GetPlayer%20HUD (Variables|Default|GetPlayerController)))))
  (Default|UpdateActionUI _aswb_stat _statcomp)
  (Default|UpdateGoldUI _aswb_stat _statcomp)
  (Default|UpdateStaminaUI _aswb_stat _statcomp)
  (Default|UpdateStatUI _aswb_stat _statcomp)
  (Default|UpdateArmorUI _aswb_stat _statcomp))

(fn PlayerMeshSelect
  (switch Utilities|FlowControl|Switch|SwitchonEPlayerMeshType (Variables|Default|GetPlayerMeshType)
    (:Badguy
      (Components|SkeletalMesh|SetSkeletalMeshAsset (Variables|Character|GetMesh) "/Game/PolygonWestern/Meshes/CharactersUE4Mannequin/SK_Chr_Badguy_01.SK_Chr_Badguy_01"))
    (:BuisinessMan
      (Components|SkeletalMesh|SetSkeletalMeshAsset (Variables|Character|GetMesh) "/Game/PolygonWestern/Meshes/CharactersUE4Mannequin/SK_Chr_Business_Man_01.SK_Chr_Business_Man_01"))
    (:Cowboy
      (Components|SkeletalMesh|SetSkeletalMeshAsset (Variables|Character|GetMesh) "/Game/PolygonWestern/Meshes/CharactersUE4Mannequin/SK_Chr_Cowboy_01.SK_Chr_Cowboy_01"))
    (:Cowgirl
      (Components|SkeletalMesh|SetSkeletalMeshAsset (Variables|Character|GetMesh) "/Game/PolygonWestern/Meshes/CharactersUE4Mannequin/SK_Chr_Cowgirl_01.SK_Chr_Cowgirl_01"))
    (:Gunman
      (Components|SkeletalMesh|SetSkeletalMeshAsset (Variables|Character|GetMesh) "/Game/PolygonWestern/Meshes/CharactersUE4Mannequin/SK_Chr_Gunman_01.SK_Chr_Gunman_01"))
    (:Sheriff
      (Components|SkeletalMesh|SetSkeletalMeshAsset (Variables|Character|GetMesh) "/Game/PolygonWestern/Meshes/CharactersUE4Mannequin/SK_Chr_Sheriff_01.SK_Chr_Sheriff_01"))
    (:Woman
      (Components|SkeletalMesh|SetSkeletalMeshAsset (Variables|Character|GetMesh) "/Game/PolygonWestern/Meshes/CharactersUE4Mannequin/SK_Chr_Woman_01.SK_Chr_Woman_01"))
    (:WorkingGirl
      (Components|SkeletalMesh|SetSkeletalMeshAsset (Variables|Character|GetMesh) "/Game/PolygonWestern/Meshes/CharactersUE4Mannequin/SK_Chr_WorkingGirl_01.SK_Chr_WorkingGirl_01"))))

(fn PlayMuzzleFlash
  (bind _righthandskeletalmesh (Variables|Default|GetRightHandSkeletalMesh))
  (Niagara|SpawnSystematLocation "/Game/StrangeShowdown/Item/FX/NS_PistolMuzzleFlash.NS_PistolMuzzleFlash" (Transformation|GetSocketLocation _righthandskeletalmesh "Muzzle") (Transformation|GetSocketRotation _righthandskeletalmesh "Muzzle")))

(fn Fire
  (Game|Damage|ApplyDamage (Variables|/Script/StrangeShowdown.STAttackTraceComponent|GetTracingFieldPlayer (Variables|Default|GetAttackTraceComp)) 1.0 0 self)
  (bind _asbp_field_player (Utilities|Casting|CastToBP_FieldPlayer (Variables|/Script/StrangeShowdown.STAttackTraceComponent|GetTracingFieldPlayer (Variables|Default|GetAttackTraceComp))))
  (Default|UpdateAllStat _asbp_field_player)
  (CallFunction|PlayMuzzleFlash)
  (Camera|PlayWorldCameraShake "/Game/StrangeShowdown/CameraShake/BP_STCameraShake.BP_STCameraShake_C" (Transformation|GetActorLocation) 0.0 5e+02)
  (Audio|SpawnSound2D "/Game/StrangeShowdown/Sound/Effect/SW_Fire.SW_Fire" 1.0 1.0 0.0 0))

(fn UseItem
  (bind (_outslot _returnvalue) (Class|STInventoryComponent|UseItem (Variables|Default|GetInventoryComp) (Utilities|Array|Get(acopy) (Variables|/Script/StrangeShowdown.STQuickSlotComponent|GetInventorySlotIndex (Variables|Default|GetQuickSlotComp)) (Variables|Default|GetCurrentSelectQuickSlotIndex)) self))
  (if _returnvalue
    (bind _returnvalue_2 (UserInterface|CreateWidget "/Game/StrangeShowdown/Item/Blueprint/WB_UseEffectFloatingMessage.WB_UseEffectFloatingMessage_C"))
    (UserInterface|Viewport|AddtoViewport _returnvalue_2 100)
    (Rendering|Components|TextRender|SetText (Variables|/Game/StrangeShowdown/Item/Blueprint/WB_UseEffectFloatingMessage.WB_UseEffectFloatingMessage_C|GetMessage _returnvalue_2) (Variables|/Script/StrangeShowdown.STItemDataAssetBase|GetItemName (.ItemData (Utilities|Struct|BreakInventorySlot _outslot))))
    (Default|UpdateQuickSlotfromUseItem (Variables|/Game/StrangeShowdown/Controller/PC_PlayerController.PC_PlayerController_C|GetPlayer%20HUD (Variables|Default|GetPlayerController)) (Variables|Default|GetQuickSlotComp))))

(fn Smash
  (Development|PrintString "망치"))