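; BP_TitlePlayer is the player character displayed for the title screen, with a selectable appearance.
; On BeginPlay it registers itself as TitlePlayer on PC_TitlePlayerController, then calls PlayerMeshSelect.
; PlayerMeshSelect switches on PlayerMeshType to swap the skeletal mesh among seven Western-style character models, and runs only if the controller cast succeeds.
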(event `self.ReceiveBeginPlay`
  (bind _aspc_title_player_controller (cast `/Game/StrangeShowdown/Controller/PC_TitlePlayerController` (`GameplayStatics.GetPlayerController` 0)))
  (set `/Game/StrangeShowdown/Controller/PC_TitlePlayerController.TitlePlayer` self _aspc_title_player_controller)
  (`self.PlayerMeshSelect`))

(fn `PlayerMeshSelect`
  (switch `EPlayerMeshType` (`self.Player Mesh Type`)
    (:`Badguy`
      (`SkeletalMeshComponent.SetSkeletalMeshAsset` (`self.Mesh`) "/Game/PolygonWestern/Meshes/CharactersUE4Mannequin/SK_Chr_Badguy_01.SK_Chr_Badguy_01"))
    (:`BusinessMan`
      (`SkeletalMeshComponent.SetSkeletalMeshAsset` (`self.Mesh`) "/Game/PolygonWestern/Meshes/CharactersUE4Mannequin/SK_Chr_Business_Man_01.SK_Chr_Business_Man_01"))
    (:`Cowboy`
      (`SkeletalMeshComponent.SetSkeletalMeshAsset` (`self.Mesh`) "/Game/PolygonWestern/Meshes/CharactersUE4Mannequin/SK_Chr_Cowboy_01.SK_Chr_Cowboy_01"))
    (:`Cowgirl`
      (`SkeletalMeshComponent.SetSkeletalMeshAsset` (`self.Mesh`) "/Game/PolygonWestern/Meshes/CharactersUE4Mannequin/SK_Chr_Cowgirl_01.SK_Chr_Cowgirl_01"))
    (:`Gunman`
      (`SkeletalMeshComponent.SetSkeletalMeshAsset` (`self.Mesh`) "/Game/PolygonWestern/Meshes/CharactersUE4Mannequin/SK_Chr_Gunman_01.SK_Chr_Gunman_01"))
    (:`Woman`
      (`SkeletalMeshComponent.SetSkeletalMeshAsset` (`self.Mesh`) "/Game/PolygonWestern/Meshes/CharactersUE4Mannequin/SK_Chr_Woman_01.SK_Chr_Woman_01"))
    (:`WorkingGirl`
      (`SkeletalMeshComponent.SetSkeletalMeshAsset` (`self.Mesh`) "/Game/PolygonWestern/Meshes/CharactersUE4Mannequin/SK_Chr_WorkingGirl_01.SK_Chr_WorkingGirl_01"))))

(fn `UserConstructionScript`
  (`parent.UserConstructionScript`))