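; Field player character that picks its skeletal mesh from a character-type enum and shows a nickname and stat widget.
; BeginPlay assigns the attack-trace widget class to the target indicator, caches the stat UI, and binds stat component changes to refresh it.
; Shift-hold handlers toggle stamina, prize and action visibility, but their controller bind and unbind nodes are disconnected, leaving EndPlay only a controller cast.
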(event `self.ReceiveEndPlay`
  (params (EndPlayReason :type "EEndPlayReason Enum" :default "Destroyed"))
  ; EndPlay
  (bind _aspc_player_controller (cast `/Game/StrangeShowdown/Controller/PC_PlayerController` (`GameplayStatics.GetPlayerController` 0))))

(event `self.ReceiveBeginPlay`
  ; BeginPlay
  (set `STTargetIndicatorComponent.AttackTraceWidgetClass` "/Game/StrangeShowdown/UI/AttackTrace/WB_AttackTrace.WB_AttackTrace_C" (`self.TargetIndicatorComponent`))
  (bind _aswb_field_player_stat_ui (cast `/Game/StrangeShowdown/UI/Interfaces/WB_FieldPlayerStatUI` (`WidgetComponent.GetUserWidgetObject` (`self.StatWidgetComponent`))))
  (set `self.StatUI` _aswb_field_player_stat_ui)
  (`self.PlayerMeshSelect`)
  (`TextBlock.SetText` (`/Game/StrangeShowdown/UI/Interfaces/WB_FieldPlayerStatUI.Nickname` (`self.StatUI`)) (`KismetTextLibrary.Conv_StringToText` (`self.PlayerNickName`)))
  (add `STStatComponent.OnStatChanged` (`self.StatComp`) (delegate `UpdateStatUI`)))

(event `OnShiftHoldStart`
  (params (IsLookingUp :type Boolean))
  ; BeginPlay
  (set `self.bOnShiftPressed` true)
  (`self.ShowShiftUI`))

(event `OnShiftHoldEnd`
  ; BeginPlay
  (set `self.bOnShiftPressed` false)
  (`self.HiddenShiftUI`))

(event `UpdateStatUI`
  (`self.UpdateAllStat`))

(fn `HiddenShiftUI`
  (`Widget.SetVisibility` (`/Game/StrangeShowdown/UI/Interfaces/WB_FieldPlayerStatUI.Stamina` (`self.StatUI`)) "Hidden")
  (`Widget.SetVisibility` (`/Game/StrangeShowdown/UI/Interfaces/WB_FieldPlayerStatUI.Prize` (`self.StatUI`)) "Hidden")
  (`Widget.SetVisibility` (`/Game/StrangeShowdown/UI/Interfaces/WB_FieldPlayerStatUI.GoldImage` (`self.StatUI`)) "Hidden")
  (`Widget.SetVisibility` (`/Game/StrangeShowdown/UI/Interfaces/WB_FieldPlayerStatUI.ActionNum` (`self.StatUI`)) "Hidden")
  (`Widget.SetVisibility` (`/Game/StrangeShowdown/UI/Interfaces/WB_FieldPlayerStatUI.ActionImage` (`self.StatUI`)) "Hidden"))

(fn `PlayerMeshSelect`
  (switch `EPlayerMeshType` (`self.PlayerMeshType`)
    (:`Badguy`
      (`SkeletalMeshComponent.SetSkeletalMeshAsset` (`self.Mesh`) "/Game/PolygonWestern/Meshes/CharactersUE4Mannequin/SK_Chr_Badguy_01.SK_Chr_Badguy_01"))
    (:`BuisinessMan`
      (`SkeletalMeshComponent.SetSkeletalMeshAsset` (`self.Mesh`) "/Game/PolygonWestern/Meshes/CharactersUE4Mannequin/SK_Chr_Business_Man_01.SK_Chr_Business_Man_01"))
    (:`Cowboy`
      (`SkeletalMeshComponent.SetSkeletalMeshAsset` (`self.Mesh`) "/Game/PolygonWestern/Meshes/CharactersUE4Mannequin/SK_Chr_Cowboy_01.SK_Chr_Cowboy_01"))
    (:`Cowgirl`
      (`SkeletalMeshComponent.SetSkeletalMeshAsset` (`self.Mesh`) "/Game/PolygonWestern/Meshes/CharactersUE4Mannequin/SK_Chr_Cowgirl_01.SK_Chr_Cowgirl_01"))
    (:`Gunman`
      (`SkeletalMeshComponent.SetSkeletalMeshAsset` (`self.Mesh`) "/Game/PolygonWestern/Meshes/CharactersUE4Mannequin/SK_Chr_Gunman_01.SK_Chr_Gunman_01"))
    (:`Woman`
      (`SkeletalMeshComponent.SetSkeletalMeshAsset` (`self.Mesh`) "/Game/PolygonWestern/Meshes/CharactersUE4Mannequin/SK_Chr_Woman_01.SK_Chr_Woman_01"))
    (:`WorkingGirl`
      (`SkeletalMeshComponent.SetSkeletalMeshAsset` (`self.Mesh`) "/Game/PolygonWestern/Meshes/CharactersUE4Mannequin/SK_Chr_WorkingGirl_01.SK_Chr_WorkingGirl_01"))))

(fn `ShowShiftUI`
  (`Widget.SetVisibility` (`/Game/StrangeShowdown/UI/Interfaces/WB_FieldPlayerStatUI.Stamina` (`self.StatUI`)) "Visible")
  (`Widget.SetVisibility` (`/Game/StrangeShowdown/UI/Interfaces/WB_FieldPlayerStatUI.Prize` (`self.StatUI`)) "Visible")
  (`Widget.SetVisibility` (`/Game/StrangeShowdown/UI/Interfaces/WB_FieldPlayerStatUI.GoldImage` (`self.StatUI`)) "Visible")
  (`Widget.SetVisibility` (`/Game/StrangeShowdown/UI/Interfaces/WB_FieldPlayerStatUI.ActionNum` (`self.StatUI`)) "Visible")
  (`Widget.SetVisibility` (`/Game/StrangeShowdown/UI/Interfaces/WB_FieldPlayerStatUI.ActionImage` (`self.StatUI`)) "Visible"))

(fn `UpdateAllStat`
  (bind _statui (`self.StatUI`))
  (bind _statcomp (`self.StatComp`))
  (`/Game/StrangeShowdown/UI/Interfaces/WB_FieldPlayerStatUI.UpdateStatUI` _statui _statcomp)
  (`/Game/StrangeShowdown/UI/Interfaces/WB_FieldPlayerStatUI.UpdatePrizeUI` _statui _statcomp)
  (`/Game/StrangeShowdown/UI/Interfaces/WB_FieldPlayerStatUI.UpdateActionUI` _statui _statcomp)
  (`/Game/StrangeShowdown/UI/Interfaces/WB_FieldPlayerStatUI.UpdateStaminaUI` _statui _statcomp))

(fn `UserConstructionScript`)