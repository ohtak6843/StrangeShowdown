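; BP_LocalPlayer is the player character Blueprint, implementing cosmetic responses to native events for pistol fire, hammer smashes, floating messages and dissolving.
; Pistol fire spawns a Niagara muzzle flash, camera shake and sound, while the hammer sets a smashing flag and plays a montage.
; A timeline drives the dissolve material parameter.
; Debug keys add stamina or gold and trigger death; victory camera and sheriff test code sit unconnected.
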(event EventPistolFire
  ;[0.15 0.15 0.15 0.5] Blueprint Implement Functions
  (CallFunction|BPFPistolFireEffect))

(event EventShowFloatingMessage
  (params (Message :type Text%20%28by%20ref%29))
  ;[0.15 0.15 0.15 0.5] Blueprint Implement Functions
  (CallFunction|BPFShowFloatingMessage Message))

(event EventPlayDissolveEffect
  (bind _dissolvetrack (Timeline|Timeline_0 PlayFromStart)
    (:Update
      (Rendering|Material|SetScalarParameterValue (Variables|Default|GetDynamicMaterial) "Dissolve" (Math|Float|Lerp -1.0 1.0 _dissolvetrack) :!class /Script/Engine.MaterialInstanceDynamic))))

(event EventHammerSmash
  ;[0.15 0.15 0.15 0.5] Blueprint Implement Functions
  (CallFunction|BPFHammerSmash))

(event Input|KeyboardEvents|DebugKey9
  (params (Key :type Key%20Structure :default "None") (ActionValue :type Input%20Action%20Value%20Structure))
  ;[0.15 0.15 0.15 0.5] Debug Key
  (:Pressed
    (Class|STLocalPlayer|AddGold 10)
    (Development|PrintString (Utilities|String|Append "Gold: " (Utilities|String|ToString(Float) (.CurrentGold (Utilities|Struct|BreakSTCharacterStat (Variables|/Script/StrangeShowdown.STStatComponent|GetCharacterStat (Variables|Default|GetStatComp)))))))))

(event Input|KeyboardEvents|DebugKey0
  (params (Key :type Key%20Structure :default "None") (ActionValue :type Input%20Action%20Value%20Structure))
  ;[0.15 0.15 0.15 0.5] Debug Key
  (:Pressed
    (Class|STLocalPlayer|AddStamina 1.0)
    (Development|PrintString (Utilities|String|Append "Stamina: " (Utilities|String|ToString(Float) (.CurrentStamina (Utilities|Struct|BreakSTCharacterStat (Variables|/Script/StrangeShowdown.STStatComponent|GetCharacterStat (Variables|Default|GetStatComp)))))))))

(event Input|KeyboardEvents|DebugKeyL
  (params (Key :type Key%20Structure :default "None") (ActionValue :type Input%20Action%20Value%20Structure))
  (:Pressed
    (Class|STPlayerBase|SetDead)
    (Development|PrintString "Hello")))

(fn ConstructionScript)

(fn PlayMuzzleFlash
  (bind _righthandskeletalmesh (Variables|Default|GetRightHandSkeletalMesh))
  (Niagara|SpawnSystematLocation "/Game/StrangeShowdown/Item/FX/NS_PistolMuzzleFlash.NS_PistolMuzzleFlash" (Transformation|GetSocketLocation _righthandskeletalmesh "Muzzle") (Transformation|GetSocketRotation _righthandskeletalmesh "Muzzle")))

(fn BPFPistolFireEffect
  (CallFunction|PlayMuzzleFlash)
  (Camera|PlayWorldCameraShake "/Game/StrangeShowdown/CameraShake/BP_CameraShake.BP_CameraShake_C" (Transformation|GetActorLocation) 0.0 5e+02)
  (Audio|SpawnSound2D "/Game/StrangeShowdown/Sound/Effect/SW_Fire.SW_Fire" 1.0 1.0 0.0 0))

(fn BPFHammerSmash
  (Variables|Default|SetIsSmashing true)
  (Animation|PlayAnimMontage "/Game/PolygonWestern/EpicContent/Mannequin/RetargetAnimations/Hammer/Great_Sword_Slash_Montage.Great_Sword_Slash_Montage" 1.0 "None"))

(fn BPFShowFloatingMessage
  (params (InText :type Text))
  (bind _returnvalue (UserInterface|CreateWidget "/Game/StrangeShowdown/UI/WB_FloatingMessage.WB_FloatingMessage_C"))
  (UserInterface|Viewport|AddtoViewport _returnvalue 100)
  (Rendering|Components|TextRender|SetText (Variables|/Game/StrangeShowdown/UI/WB_FloatingMessage.WB_FloatingMessage_C|GetMessage _returnvalue) InText))