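; Temporary local player character for the Strange Showdown lobby, with basic movement, look controls and a selectable appearance.
; On BeginPlay it requires a PC_LobbyController, adds the Enhanced Input mapping context, then runs PlayerMeshSelect.
; PlayerMeshSelect swaps the skeletal mesh by PlayerMeshType among Western-style character models.
; Input actions drive controller yaw and inverted pitch, plus movement relative to control rotation.
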(event `self.ReceiveBeginPlay`
  ; BeginPlay
  (bind _aspc_lobby_controller (cast `/Game/StrangeShowdown/Controller/PC_LobbyController` (`self.GetController`)))
  (bind _output_get (set `self.PlayerController` _aspc_lobby_controller))
  (message `EnhancedInputSubsystemInterface.AddMappingContext` (pcsubsystem `EnhancedInputLocalPlayerSubsystem` _output_get) "/Game/StrangeShowdown/Input/IMC_PlayerInput.IMC_PlayerInput" 0 (struct))
  (`self.PlayerMeshSelect`))

(event `EnhancedInput|/Game/StrangeShowdown/Input/Actions/IA_LookAround`
  (params (ActionValue :type "Vector2D Structure") (ElapsedSeconds :type "Float (double-precision)") (TriggeredSeconds :type "Float (double-precision)") (InputAction :type "InputAction Object Reference" :default "/Game/StrangeShowdown/Input/Actions/IA_LookAround.IA_LookAround"))
  ; IA_LookAround
  (:`Triggered`
    (`self.AddControllerYawInput` ActionValue_X)
    (`self.AddControllerPitchInput` (* ActionValue_Y -1.0))))

(event `EnhancedInput|/Game/StrangeShowdown/Input/Actions/IA_Movement`
  (params (ActionValue :type "Vector2D Structure") (ElapsedSeconds :type "Float (double-precision)") (TriggeredSeconds :type "Float (double-precision)") (InputAction :type "InputAction Object Reference" :default "/Game/StrangeShowdown/Input/Actions/IA_Movement.IA_Movement"))
  (bind (_returnvalue_roll _returnvalue_pitch _returnvalue_yaw) (`KismetMathLibrary.BreakRotator` (`self.GetControlRotation`)))
  (bind (_returnvalue_roll_2 _returnvalue_pitch_2 _returnvalue_yaw_2) (`KismetMathLibrary.BreakRotator` (`self.GetControlRotation`)))
  ; IA_Movement
  (:`Triggered`
    (`self.AddMovementInput` (`KismetMathLibrary.GetRightVector` (`KismetMathLibrary.MakeRotator` _returnvalue_roll_2 0.0 _returnvalue_yaw_2)) ActionValue_X)
    (`self.AddMovementInput` (`KismetMathLibrary.GetForwardVector` (`KismetMathLibrary.MakeRotator` 0.0 0.0 _returnvalue_yaw)) ActionValue_Y)))

(fn `PlayerMeshSelect`
  (switch `EPlayerMeshType` (`self.PlayerMeshType`)
    (:`Badguy`
      (`SkeletalMeshComponent.SetSkeletalMeshAsset` (`self.Mesh`) "/Game/PolygonWestern/Meshes/CharactersUE4Mannequin/SK_Chr_Badguy_01.SK_Chr_Badguy_01"))
    (:`BuisinessMan`
      (`SkeletalMeshComponent.SetSkeletalMeshAsset` (`self.Mesh`) "/Game/PolygonWestern/Meshes/CharactersUE4Mannequin/SK_Chr_Business_Man_01.SK_Chr_Business_Man_01"))
    (:`Cowboy`
      (`SkeletalMeshComponent.SetSkeletalMeshAsset` (`self.Mesh`) "/Game/PolygonWestern/Meshes/CharactersUE4Mannequin/SK_Chr_Cowboy_01.SK_Chr_Cowboy_01"))
    (:`Cowgirl`
      (`SkeletalMeshComponent.SetSkeletalMeshAsset` (`self.Mesh`) "/Game/PolygonWestern/Meshes/CharactersUE4Mannequin/SK_Chr_Cowgirl_01.SK_Chr_Cowgirl_01"))
    (:`Gunman`
      (`SkeletalMeshComponent.SetSkeletalMeshAsset` (`self.Mesh`) "/Game/PolygonWestern/Meshes/CharactersUE4Mannequin/SK_Chr_Gunman_01.SK_Chr_Gunman_01"))
    (:`Woman`
      (`SkeletalMeshComponent.SetSkeletalMeshAsset` (`self.Mesh`) "/Game/PolygonWestern/Meshes/CharactersUE4Mannequin/SK_Chr_Woman_01.SK_Chr_Woman_01"))
    (:`WorkingGirl`
      (`SkeletalMeshComponent.SetSkeletalMeshAsset` (`self.Mesh`) "/Game/PolygonWestern/Meshes/CharactersUE4Mannequin/SK_Chr_WorkingGirl_01.SK_Chr_WorkingGirl_01"))))

(fn `UserConstructionScript`)