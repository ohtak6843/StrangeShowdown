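; Local player's Sheriff character Blueprint, which drives the HUD through PC_SheriffController.
; BeginPlay sets the HUD to its Sheriff type, clears quick-slot selection since the Sheriff doesn't use slots, and gives each slot the Sheriff image.
; Stat updates push StatComp values into the stat widget, then refresh the Tab menu if valid.
; InitHUD, also bound to debug key Z, resets the HUD and refreshes stats.
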(event Custom|InitHUD
  ;[0.15 0.15 0.15 0.5] Initialize HUD
  (Default|ResetHUD (Variables|/Game/StrangeShowdown/Controller/PC_SheriffController.PC_SheriffController_C|GetPlayer%20HUD (Variables|Default|GetSheriff%20Controller)))
  (CallFunction|InitializeStatUI))

(event Custom|InitializeQuickSlot
  ;[0.15 0.15 0.15 0.5] InitializeQuickSlot
  (Default|InitializeQuickSlot (Variables|/Game/StrangeShowdown/Controller/PC_SheriffController.PC_SheriffController_C|GetPlayer%20HUD (Variables|Default|GetSheriff%20Controller)) (Variables|Default|GetQuickSlotComp)))

(event Custom|InitializeStatUI
  (bind _sheriff_controller (Variables|Default|GetSheriff%20Controller))
  (bind _player_hud (Variables|/Game/StrangeShowdown/Controller/PC_SheriffController.PC_SheriffController_C|GetPlayer%20HUD _sheriff_controller))
  (bind _wb_tabuimenu (Variables|/Game/StrangeShowdown/UI/WB_HUD.WB_HUD_C|GetWB_TabUIMenu _player_hud))
  ;[0.15 0.15 0.15 0.5] Stat UI
  (CallFunction|UpdateAllStat) ; 자신의 UI
  (Utilities|IsValid _wb_tabuimenu
    (:Is%20Valid
      (Default|UpdateTabUI (Variables|/Game/StrangeShowdown/UI/TabUI/WB_TabUIMenu.WB_TabUIMenu_C|GetWB_TabUI _wb_tabuimenu)) ; Update Stat UI 이벤트가 호출되면\nTab UI도 새로 만들어 업데이트를 처리함
    )))

(event Custom|UpdateStatUI
  (bind _sheriff_controller (Variables|Default|GetSheriff%20Controller))
  (bind _player_hud (Variables|/Game/StrangeShowdown/Controller/PC_SheriffController.PC_SheriffController_C|GetPlayer%20HUD _sheriff_controller))
  (bind _wb_tabuimenu (Variables|/Game/StrangeShowdown/UI/WB_HUD.WB_HUD_C|GetWB_TabUIMenu _player_hud))
  ;[0.15 0.15 0.15 0.5] Stat UI
  (CallFunction|UpdateAllStat) ; 자신의 UI
  (Utilities|IsValid _wb_tabuimenu
    (:Is%20Valid
      (Default|UpdateTabUI (Variables|/Game/StrangeShowdown/UI/TabUI/WB_TabUIMenu.WB_TabUIMenu_C|GetWB_TabUI _wb_tabuimenu)) ; Update Stat UI 이벤트가 호출되면\nTab UI도 새로 만들어 업데이트를 처리함
    )))

(event EventBeginPlay
  ;[0.15 0.15 0.15 0.5] Begin Play
  (bind _aspc_sheriff_controller (Utilities|Casting|CastToPC_SheriffController (Pawn|GetController)))
  (bind _output_get (Variables|Default|SetSheriff%20Controller _aspc_sheriff_controller))
  (Variables|/Script/StrangeShowdown.STHUD|SetHUDWidgetType (Variables|/Game/StrangeShowdown/Controller/PC_SheriffController.PC_SheriffController_C|GetPlayer%20HUD _output_get) "Sheriff")
  (Variables|/Script/StrangeShowdown.STQuickSlotComponent|SetCurrentSelectQuickSlotIndex (Variables|Default|GetQuickSlotComp) -1) ; 보안관은 퀵슬롯은 안쓰므로 -1
  (CallFunction|InitializeQuickSlot)
  (for _index (range 0 (Class|PanelWidget|GetChildrenCount (Variables|/Game/StrangeShowdown/UI/WB_HUD.WB_HUD_C|GetQuickSlots (Variables|/Game/StrangeShowdown/Controller/PC_SheriffController.PC_SheriffController_C|GetPlayer%20HUD _output_get))))
    (bind _aswb_quick_slot (Utilities|Casting|CastToWB_QuickSlot (Class|PanelWidget|GetChildat (Variables|/Game/StrangeShowdown/UI/WB_HUD.WB_HUD_C|GetQuickSlots (Variables|/Game/StrangeShowdown/Controller/PC_SheriffController.PC_SheriffController_C|GetPlayer%20HUD _output_get)) _index)))
    (Default|SetSheriffImage _aswb_quick_slot)
    (CallFunction|InitializeStatUI)))

(event Input|KeyboardEvents|DebugKeyZ
  (params (Key :type Key%20Structure :default "None") (ActionValue :type Input%20Action%20Value%20Structure))
  ;[0.15 0.15 0.15 0.5] Initialize HUD
  (:Pressed
    (Default|ResetHUD (Variables|/Game/StrangeShowdown/Controller/PC_SheriffController.PC_SheriffController_C|GetPlayer%20HUD (Variables|Default|GetSheriff%20Controller)))
    (CallFunction|InitializeStatUI)))

(fn ConstructionScript)

(fn UpdateAllStat
  (bind _statcomp (Variables|Default|GetStatComp))
  (bind _aswb_stat (Utilities|Casting|CastToWB_Stat (Variables|/Script/StrangeShowdown.STHUD|GetStatWidget (Variables|/Game/StrangeShowdown/Controller/PC_SheriffController.PC_SheriffController_C|GetPlayer%20HUD (Variables|Default|GetSheriff%20Controller)))))
  (Default|UpdateActionUI _aswb_stat _statcomp)
  (Default|UpdateGoldUI _aswb_stat _statcomp)
  (Default|UpdateStaminaUI _aswb_stat _statcomp)
  (Default|UpdateStatUI _aswb_stat _statcomp)
  (Default|UpdateArmorUI _aswb_stat _statcomp))