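; Mineable mineral prop that gives gold feedback and shatters in stages through three Blueprint events, each receiving a Gold amount.
; Every event shows a floating gold-gained message and plays a hit or break sound.
; The sliced events swap a mesh for its physics-simulated geometry collection, then after a short delay hide the debris and disable collision.
; OnSubSliced breaks MeshComponent, while OnMainSliced breaks SubMineralMeshComponent and destroys the actor.
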(event `self.OnSubSlicedBlueprint`
  (params (gold :type Integer))
  (bind _gc_mineral (`self.GC_Mineral`))
  (bind _returnvalue (`|CreateWidget` "/Game/StrangeShowdown/UI/WB_FloatingMessage.WB_FloatingMessage_C"))
  (`UserWidget.AddToViewport` _returnvalue 100)
  (`TextBlock.SetText` (`/Game/StrangeShowdown/UI/WB_FloatingMessage.Message` _returnvalue) (`KismetTextLibrary.Conv_StringToText` (`KismetStringLibrary.Concat_StrStr` (`KismetStringLibrary.Conv_IntToString` gold) "골드 획득!")))
  (`SceneComponent.SetVisibility` (`self.MeshComponent`) false false)
  (`GameplayStatics.SpawnSound2D` "/Game/StrangeShowdown/Sound/Effect/SW_MineralBreak.SW_MineralBreak" 1.0 1.0 0.1 null)
  (`SceneComponent.SetHiddenInGame` _gc_mineral false false)
  (`GeometryCollectionComponent.SetEnableDamageFromCollision` _gc_mineral true)
  (`PrimitiveComponent.SetSimulatePhysics` _gc_mineral true)
  (`KismetSystemLibrary.Delay` 2.0)
  (`SceneComponent.SetHiddenInGame` (`self.GC_Mineral`) true false)
  (`PrimitiveComponent.SetCollisionEnabled` (`self.MeshComponent`) "NoCollision")
  (`PrimitiveComponent.SetCollisionEnabled` (`self.GC_Mineral`) "NoCollision"))

(event `self.OnMainSlicedBlueprint`
  (params (gold :type Integer))
  (bind _gc_submineral (`self.GC_SubMineral`))
  (bind _returnvalue (`|CreateWidget` "/Game/StrangeShowdown/UI/WB_FloatingMessage.WB_FloatingMessage_C"))
  (`UserWidget.AddToViewport` _returnvalue 100)
  (`TextBlock.SetText` (`/Game/StrangeShowdown/UI/WB_FloatingMessage.Message` _returnvalue) (`KismetTextLibrary.Conv_StringToText` (`KismetStringLibrary.Concat_StrStr` (`KismetStringLibrary.Conv_IntToString` gold) "골드 획득!")))
  (`SceneComponent.SetVisibility` (`self.SubMineralMeshComponent`) false false)
  (`GameplayStatics.SpawnSound2D` "/Game/StrangeShowdown/Sound/Effect/SW_MineralBreak.SW_MineralBreak" 1.0 1.0 0.1 null)
  (`SceneComponent.SetHiddenInGame` _gc_submineral false false)
  (`GeometryCollectionComponent.SetEnableDamageFromCollision` _gc_submineral true)
  (`PrimitiveComponent.SetSimulatePhysics` _gc_submineral true)
  (`KismetSystemLibrary.Delay` 2.0)
  (`PrimitiveComponent.SetSimulatePhysics` _gc_submineral false)
  (`SceneComponent.SetHiddenInGame` (`self.GC_SubMineral`) true false)
  (`PrimitiveComponent.SetCollisionEnabled` (`self.SubMineralMeshComponent`) "NoCollision")
  (`PrimitiveComponent.SetCollisionEnabled` (`self.GC_SubMineral`) "NoCollision")
  (`self.K2_DestroyActor`))

(event `self.OnHitSoundBlueprint`
  (params (gold :type Integer))
  (bind _returnvalue (`|CreateWidget` "/Game/StrangeShowdown/UI/WB_FloatingMessage.WB_FloatingMessage_C"))
  (`UserWidget.AddToViewport` _returnvalue 100)
  (`TextBlock.SetText` (`/Game/StrangeShowdown/UI/WB_FloatingMessage.Message` _returnvalue) (`KismetTextLibrary.Conv_StringToText` (`KismetStringLibrary.Concat_StrStr` (`KismetStringLibrary.Conv_IntToString` gold) "골드 획득!")))
  (`GameplayStatics.SpawnSound2D` "/Game/StrangeShowdown/Sound/Effect/SW_MineralHit.SW_MineralHit" 1.0 1.0 0.1 null))

(fn `UserConstructionScript`)