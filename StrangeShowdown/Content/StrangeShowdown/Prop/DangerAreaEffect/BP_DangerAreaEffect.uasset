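; BP_DangerAreaEffect is a looping visual effect prop, named for marking danger areas, built on three plane meshes that continually rise.
; Each Tick passes every plane to MoveLocation, which lifts it at a constant, frame-rate-independent speed and snaps it back to zero height at an upper limit.
; Both heights are absolute world Z, so the loop ignores the actor's own elevation.
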(event `self.ReceiveTick`
  (params (DeltaSeconds :type "Float (single-precision)"))
  (`self.MoveLocation` (`self.Plane`) DeltaSeconds)
  (`self.MoveLocation` (`self.Plane1`) DeltaSeconds)
  (`self.MoveLocation` (`self.Plane2`) DeltaSeconds))

(fn `MoveLocation`
  (params (StaticMesh :type "SceneComponent Object Reference") (DeltaSecond :type "Float (double-precision)"))
  (bind _x (.x (`SceneComponent.K2_GetComponentLocation` StaticMesh)))
  (bind _y (.y (`SceneComponent.K2_GetComponentLocation` StaticMesh)))
  (bind _returnvalue (+ (.z (`SceneComponent.K2_GetComponentLocation` StaticMesh)) (* DeltaSecond 60.0)))
  (if (>= _returnvalue 200.0)
    (`SceneComponent.K2_SetWorldLocation` StaticMesh (`KismetMathLibrary.MakeVector` _x _y) false false)
    (else
      (`SceneComponent.K2_SetWorldLocation` StaticMesh (`KismetMathLibrary.MakeVector` _x _y _returnvalue) false false))))

(fn `UserConstructionScript`)