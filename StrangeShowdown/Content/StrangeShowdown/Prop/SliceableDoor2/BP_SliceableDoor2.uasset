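; BP_SliceableDoor2 is a wooden door prop that breaks apart when sliced.
; On slice it hides the intact mesh, plays a wood-break sound, and reveals the GCSliceableDoor2 component with physics and collision damage enabled.
; After a short delay it hides the broken pieces and disables collision on both components, leaving the actor in place.
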(event `self.OnSlicedBlueprint`
  (bind _gc_sliceabledoor2 (`self.GC_SliceableDoor2`))
  (`SceneComponent.SetVisibility` (`self.MeshComponent`) false false)
  (`GameplayStatics.SpawnSound2D` "/Game/StrangeShowdown/Sound/Effect/SW_WoodBreak.SW_WoodBreak" 1.0 1.0 0.1 null)
  (`SceneComponent.SetHiddenInGame` _gc_sliceabledoor2 false false)
  (`GeometryCollectionComponent.SetEnableDamageFromCollision` _gc_sliceabledoor2 true)
  (`PrimitiveComponent.SetSimulatePhysics` _gc_sliceabledoor2 true)
  (`KismetSystemLibrary.Delay` 1.0)
  (`SceneComponent.SetHiddenInGame` (`self.GC_SliceableDoor2`) true false)
  (`PrimitiveComponent.SetCollisionEnabled` (`self.MeshComponent`) "NoCollision")
  (`PrimitiveComponent.SetCollisionEnabled` (`self.GC_SliceableDoor2`) "NoCollision"))

(fn `UserConstructionScript`)