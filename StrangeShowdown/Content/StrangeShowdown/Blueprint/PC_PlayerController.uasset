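; PC_PlayerController is a player controller that owns the player's HUD and toggles the inventory menu.
; On BeginPlay it creates the WB_HUD widget, stores it as PlayerHUD and adds it to the viewport.
; Each start of the IA_Inventory input action alternates through a FlipFlop, telling the HUD to show or remove the inventory menu and updating IsInventoryOpen to match.
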(event `self.ReceiveBeginPlay`
  (bind _returnvalue (`|CreateWidget` "/Game/StrangeShowdown/UI/WB_HUD.WB_HUD_C"))
  (bind _output_get (set `self.Player HUD` _returnvalue))
  (`UserWidget.AddToViewport` _output_get 0))

(event `EnhancedInput|/Game/StrangeShowdown/Input/Actions/IA_Inventory`
  (params (ActionValue :type Boolean) (ElapsedSeconds :type "Float (double-precision)") (TriggeredSeconds :type "Float (double-precision)") (InputAction :type "InputAction Object Reference" :default "/Game/StrangeShowdown/Input/Actions/IA_Inventory.IA_Inventory"))
  (:`Started`
    (`/Engine/EditorBlueprintResources/StandardMacros.FlipFlop`
      (:`A`
        (`/Game/StrangeShowdown/UI/WB_HUD.ShowInventoryMenu` (`self.Player HUD`))
        (set `self.IsInventoryOpen` true))
      (:`B`
        (`/Game/StrangeShowdown/UI/WB_HUD.RemoveInventoryMenu` (`self.Player HUD`))
        (set `self.IsInventoryOpen` false)))))

(fn `UserConstructionScript`)