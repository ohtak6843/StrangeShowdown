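; BP_LocalPlayerBase is the base Blueprint for the locally controlled player, handling look, movement and item pickup.
; On BeginPlay it caches the PC_PlayerController, adds the Enhanced Input mapping context and hands its quick slot component to the HUD.
; Look input drives controller yaw and inverted pitch, while movement follows control rotation.
; Pickup calls Interact, then refreshes the HUD menu's inventory widget from the inventory component if the menu exists.
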(event `self.ReceiveBeginPlay`
  ; CastToPlayerController
  (bind _aspc_player_controller (cast `/Game/StrangeShowdown/Blueprint/PC_PlayerController` (`self.GetController`)))
  (bind _output_get (set `self.PlayerController` _aspc_player_controller))
  (message `EnhancedInputSubsystemInterface.AddMappingContext` (pcsubsystem `EnhancedInputLocalPlayerSubsystem` _output_get) "/Game/StrangeShowdown/Input/IMC_PlayerBaseInput.IMC_PlayerBaseInput" 0 (struct))
  (`self.InitializeQuickSlot`))

(event `EnhancedInput|/Game/StrangeShowdown/Input/Actions/IA_LookAround`
  (params (ActionValue :type "Vector2D Structure") (ElapsedSeconds :type "Float (double-precision)") (TriggeredSeconds :type "Float (double-precision)") (InputAction :type "InputAction Object Reference" :default "/Game/StrangeShowdown/Input/Actions/IA_LookAround.IA_LookAround"))
  ; IA_LookAround
  (:`Triggered`
    (`self.AddControllerYawInput` ActionValue_X)
    (`self.AddControllerPitchInput` (* ActionValue_Y -1.0))))

(event `EnhancedInput|/Game/StrangeShowdown/Input/Actions/IA_Movement`
  (params (ActionValue :type "Vector2D Structure") (ElapsedSeconds :type "Float (double-precision)") (TriggeredSeconds :type "Float (double-precision)") (InputAction :type "InputAction Object Reference" :default "/Game/StrangeShowdown/Input/Actions/IA_Movement.IA_Movement"))
  (bind (_returnvalue_roll _returnvalue_pitch _returnvalue_yaw) (`KismetMathLibrary.BreakRotator` (`self.GetControlRotation`)))
  (bind (_returnvalue_roll_2 _returnvalue_pitch_2 _returnvalue_yaw_2) (`KismetMathLibrary.BreakRotator` (`self.GetControlRotation`)))
  ; IA_Movement
  (:`Triggered`
    (`self.AddMovementInput` (`KismetMathLibrary.GetRightVector` (`KismetMathLibrary.MakeRotator` _returnvalue_roll_2 0.0 _returnvalue_yaw_2)) ActionValue_X)
    (`self.AddMovementInput` (`KismetMathLibrary.GetForwardVector` (`KismetMathLibrary.MakeRotator` 0.0 0.0 _returnvalue_yaw)) ActionValue_Y)))

(event `EnhancedInput|/Game/StrangeShowdown/Input/Actions/IA_Pickup`
  (params (ActionValue :type Boolean) (ElapsedSeconds :type "Float (double-precision)") (TriggeredSeconds :type "Float (double-precision)") (InputAction :type "InputAction Object Reference" :default "/Game/StrangeShowdown/Input/Actions/IA_Pickup.IA_Pickup"))
  ; IA_Pickup
  (:`Triggered`
    (`self.Interact`)
    (`self.UpdateInventory`)))

(event `UpdateInventory`
  (bind _wb_menu (`/Game/StrangeShowdown/UI/WB_HUD.WB_Menu` (`/Game/StrangeShowdown/Blueprint/PC_PlayerController.Player HUD` (`self.PlayerController`))))
  (`/Engine/EditorBlueprintResources/StandardMacros.IsValid` _wb_menu
    (:`Is Valid`
      (`/Game/StrangeShowdown/UI/Inventory/WB_Inventory.UpdateInventory` (`/Game/StrangeShowdown/UI/Inventory/WB_InventoryMenu.WB_Inventory` _wb_menu) (`self.InventoryComp`)))))

(event `InitializeQuickSlot`
  (`/Game/StrangeShowdown/UI/WB_HUD.InitializeQuickSlot` (`/Game/StrangeShowdown/Blueprint/PC_PlayerController.Player HUD` (`self.PlayerController`)) (`self.QuickSlot Comp`)))

(fn `UserConstructionScript`)