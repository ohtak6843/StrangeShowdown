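; BP_PlayerBase is the base player pawn Blueprint, providing Enhanced Input look and movement.
; On BeginPlay it casts its controller to STPlayerController and adds the IMC_PlayerBaseInput mapping context.
; IA_LookAround drives controller yaw and inverted pitch.
; IA_Movement feeds movement input along control-rotation axes with pitch zeroed, keeping forward motion horizontal.
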(event `self.ReceiveBeginPlay`
  ; CastToPlayerController
  (bind _asstplayer_controller (cast `STPlayerController` (`self.GetController`)))
  (message `EnhancedInputSubsystemInterface.AddMappingContext` (pcsubsystem `EnhancedInputLocalPlayerSubsystem` _asstplayer_controller) "/Game/Input/IMC_PlayerBaseInput.IMC_PlayerBaseInput" 0 (struct)))

(event `EnhancedInput|/Game/Input/IA_LookAround`
  (params (ActionValue :type "Vector2D Structure") (ElapsedSeconds :type "Float (double-precision)") (TriggeredSeconds :type "Float (double-precision)") (InputAction :type "InputAction Object Reference" :default "/Game/Input/IA_LookAround.IA_LookAround"))
  ; IA_LookAround
  (:`Triggered`
    (`self.AddControllerYawInput` ActionValue_X)
    (`self.AddControllerPitchInput` (* ActionValue_Y -1.0))))

(event `EnhancedInput|/Game/Input/IA_Movement`
  (params (ActionValue :type "Vector2D Structure") (ElapsedSeconds :type "Float (double-precision)") (TriggeredSeconds :type "Float (double-precision)") (InputAction :type "InputAction Object Reference" :default "/Game/Input/IA_Movement.IA_Movement"))
  (bind (_returnvalue_roll _returnvalue_pitch _returnvalue_yaw) (`KismetMathLibrary.BreakRotator` (`self.GetControlRotation`)))
  (bind (_returnvalue_roll_2 _returnvalue_pitch_2 _returnvalue_yaw_2) (`KismetMathLibrary.BreakRotator` (`self.GetControlRotation`)))
  ; IA_Movement
  (:`Triggered`
    (`self.AddMovementInput` (`KismetMathLibrary.GetRightVector` (`KismetMathLibrary.MakeRotator` _returnvalue_roll_2 0.0 _returnvalue_yaw_2)) ActionValue_X)
    (`self.AddMovementInput` (`KismetMathLibrary.GetForwardVector` (`KismetMathLibrary.MakeRotator` 0.0 0.0 _returnvalue_yaw)) ActionValue_Y)))

(fn `UserConstructionScript`)